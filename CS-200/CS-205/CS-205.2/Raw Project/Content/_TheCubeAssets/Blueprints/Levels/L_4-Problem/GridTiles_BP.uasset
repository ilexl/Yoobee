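; GridTiles_BP is a level grid tile that hurts the player on contact unless it has been shot first.
; The Cube's hit event branches on the other actor, using the tile's current material as its state.
; A first-person character hitting a default hex tile takes damage, turns it pulsing red, and the tile is destroyed after a short delay.
; A projectile hit swaps in the pulse material, which skips that damage check.
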(event OnComponentHit(Cube)
  (params (HitComponent :type Primitive%20Component%20Object%20Reference) (OtherActor :type Actor%20Object%20Reference) (OtherComp :type Primitive%20Component%20Object%20Reference) (NormalImpulse :type Vector :default "0, 0, 0") (Hit :type Hit%20Result%20Structure%20%28by%20ref%29))
  ;[1 1 1] When player touches Brown platform take 1 Damage
  (bind _asbp_first_person_character (Utilities|Casting|CastToBP_FirstPersonCharacter OtherActor)
    (:then
      (Utilities|Casting|CastToGridTiles_BP self)
      (if (== (Rendering|Material|GetMaterial (Variables|Default|GetCube) 0) "/Game/StarterContent/Materials/M_Tech_Hex_Tile.M_Tech_Hex_Tile")
        (Default|TakeDamage _asbp_first_person_character 1.0)
        (Rendering|Material|SetMaterial (Variables|Default|GetCube) 0 "/Game/StarterContent/Materials/M_Tech_Hex_Tile_PulseRed.M_Tech_Hex_Tile_PulseRed")
        ;[1 1 1] Destroy Brown cube after delay
        (Utilities|FlowControl|Delay 2.0)
        (Actor|DestroyActor)))
    (:CastFailed
      ;[1 1 1] Set Material When Shot
      (Utilities|Casting|CastToBP_FirstPersonProjectile OtherActor)
      (Rendering|Material|SetMaterial (Variables|Default|GetCube) 0 "/Game/StarterContent/Materials/M_Tech_Hex_Tile_Pulse.M_Tech_Hex_Tile_Pulse"))))

(fn ConstructionScript)