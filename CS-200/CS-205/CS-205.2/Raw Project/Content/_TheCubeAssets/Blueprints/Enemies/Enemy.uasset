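; Enemy actor with health, a widget health bar, a function to damage the first-person player, and a helper mapping LevelManager's current level to a colour material.
; RecieveDamage updates the bar and sets Dead at zero health, which Tick polls to run KillThis.
; KillThis uses LootQ to roll loot once, randomly spawning health or either weapon's ammo attached to a Blank actor, then destroys the enemy, with a placeholder print for death sound.
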(event EventBeginPlay
  (CallFunction|UpdateHealth)
  (Variables|Default|SetDead false))

(event Collision|EventActorBeginOverlap
  (params (OtherActor :type Actor%20Object%20Reference)))

(event EventTick
  (params (DeltaSeconds :type Float%20%28single-precision%29))
  (if (Variables|Default|GetDead)
    (CallFunction|KillThis)))

(fn ConstructionScript)

(fn RecieveDamage
  (params (Damage :type Float%20%28double-precision%29))
  (bind _output_get (Variables|Default|SetHealth (- (Variables|Default|GetHealth) Damage)))
  (CallFunction|UpdateHealth)
  (if (<= _output_get 0.0)
    (Variables|Default|SetDead true)))

(fn DamagePlayer
  (params (Damage :type Float%20%28double-precision%29))
  (bind _returnvalue (Actor|GetActorOfClass "/Game/_TheCubeAssets/Blueprints/Player/Blueprints/BP_FirstPersonCharacter.BP_FirstPersonCharacter_C"))
  (Default|TakeDamage _returnvalue Damage))

(fn KillThis
  (if (Utilities|IsValid self)
    (if (Variables|Default|GetLootQ)
      ;[0.9325 0 1] Debug
      (Development|PrintString "Kill enemy sound effect required" true true "(R=1.000000,G=0.537990,B=0.000000,A=1.000000)" :!label _label)
      (Development|PrintString (Utilities|String|Append "INFO: Enemy killed --" (Utilities|GetObjectName self)) true true "(R=0.111478,G=1.000000,B=0.000000,A=1.000000)")
      (Actor|DestroyActor)
      (else
        (Variables|Default|SetLootQ true)
        ;[0 1 0.6082] Spawn a pickup randomly when dead
        (switch int (Math|Random|RandomIntegerinRange 1 6)
          (:Default
            (goto _label))
          (:1
            (bind _returnvalue (Game|SpawnActorfromClass "/Game/_TheCubeAssets/Blueprints/Items/BP_Health.BP_Health_C" (Transformation|GetActorTransform self) "AlwaysSpawn" "MultiplyWithRoot" 0 0))
            (bind _returnvalue_2 (Actor|GetActorOfClass "/Game/_TheCubeAssets/Blueprints/Levels/Blank.Blank_C"))
            (if (Utilities|IsValid _returnvalue)
              (Transformation|AttachActorToActor _returnvalue _returnvalue_2 "None" "KeepWorld" "KeepWorld" "KeepWorld" false)
              (goto _label)))
          (:3
            (bind _returnvalue_3 (Game|SpawnActorfromClass "/Game/_TheCubeAssets/Blueprints/Items/BP_Ammo_Weapon1.BP_Ammo_Weapon1_C" (Transformation|GetActorTransform self) "AlwaysSpawn" "MultiplyWithRoot" 0 0))
            (bind _returnvalue_4 (Actor|GetActorOfClass "/Game/_TheCubeAssets/Blueprints/Levels/Blank.Blank_C"))
            (if (Utilities|IsValid _returnvalue_3)
              (Transformation|AttachActorToActor _returnvalue_3 _returnvalue_4 "None" "KeepWorld" "KeepWorld" "KeepWorld" false)
              (goto _label)))
          (:5
            (bind _returnvalue_5 (Game|SpawnActorfromClass "/Game/_TheCubeAssets/Blueprints/Items/BP_Ammo_Weapon2.BP_Ammo_Weapon2_C" (Transformation|GetActorTransform self) "AlwaysSpawn" "MultiplyWithRoot" 0 0))
            (bind _returnvalue_6 (Actor|GetActorOfClass "/Game/_TheCubeAssets/Blueprints/Levels/Blank.Blank_C"))
            (if (Utilities|IsValid _returnvalue_5)
              (Transformation|AttachActorToActor _returnvalue_5 _returnvalue_6 "None" "KeepWorld" "KeepWorld" "KeepWorld" false)
              (goto _label))))))))

(fn UpdateHealth
  (bind _aswbp_health_bar (Utilities|Casting|CastToWBP_HealthBar (UserInterface|GetUserWidgetObject (Variables|Default|GetWidget))))
  (Variables|/Game/_TheCubeAssets/Blueprints/Enemies/WBP_HealthBar.WBP_HealthBar_C|SetHealth _aswbp_health_bar (/ (Variables|Default|GetHealth) (Variables|Default|GetMaxHealth)))
  (return))

(fn GetCurrentLevel+Colour
  (bind _returnvalue (Actor|GetActorOfClass "/Game/_TheCubeAssets/Blueprints/LevelManager.LevelManager_C"))
  (switch int (Variables|/Game/_TheCubeAssets/Blueprints/LevelManager.LevelManager_C|GetLevel%20To%20Play _returnvalue)
    (:Default
      (return "/Game/_TheCubeAssets/Materials/BasicSolids/M_Solid_White.M_Solid_White" (Variables|/Game/_TheCubeAssets/Blueprints/LevelManager.LevelManager_C|GetLevel%20To%20Play _returnvalue)))
    (:0
      (return "/Game/_TheCubeAssets/Materials/BasicSolids/M_Solid_Blue.M_Solid_Blue" (Variables|/Game/_TheCubeAssets/Blueprints/LevelManager.LevelManager_C|GetLevel%20To%20Play _returnvalue)))
    (:1
      (return "/Game/_TheCubeAssets/Materials/BasicSolids/M_Solid_Green.M_Solid_Green" (Variables|/Game/_TheCubeAssets/Blueprints/LevelManager.LevelManager_C|GetLevel%20To%20Play _returnvalue)))
    (:2
      (return "/Game/_TheCubeAssets/Materials/BasicSolids/M_Solid_Orange.M_Solid_Orange" (Variables|/Game/_TheCubeAssets/Blueprints/LevelManager.LevelManager_C|GetLevel%20To%20Play _returnvalue)))
    (:3
      (return "/Game/_TheCubeAssets/Materials/BasicSolids/M_Solid_Purple.M_Solid_Purple" (Variables|/Game/_TheCubeAssets/Blueprints/LevelManager.LevelManager_C|GetLevel%20To%20Play _returnvalue)))
    (:4
      (return "/Game/_TheCubeAssets/Materials/BasicSolids/M_Solid_Red.M_Solid_Red" (Variables|/Game/_TheCubeAssets/Blueprints/LevelManager.LevelManager_C|GetLevel%20To%20Play _returnvalue)))
    (:5
      (return "/Game/_TheCubeAssets/Materials/BasicSolids/M_Solid_Yellow.M_Solid_Yellow" (Variables|/Game/_TheCubeAssets/Blueprints/LevelManager.LevelManager_C|GetLevel%20To%20Play _returnvalue)))))