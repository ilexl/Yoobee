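; Player weapon manager that switches between unarmed, rifle and minigun by number keys or Tab and tracks magazine and reserve ammo for each gun.
; WeaponSelect clears the current weapon and its input mapping, then adds a rifle component to the first-person character or spawns and attaches a Minigun actor.
; Reload and the AddAmmo functions update the counts and push text to the HUD through the game instance.
; Slot 3 is an unimplemented placeholder.
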(event EventBeginPlay
  (Variables|Default|SetWeapon%20Selection 4)
  (bind _output_get (Variables|Default|SetMagSizeWeapon1 30))
  (Variables|Default|SetCurrentMagWeapon1 _output_get)
  (Variables|Default|SetRemainingAmmoWeapon1 90)
  (bind _output_get_2 (Variables|Default|SetMagSizeWeapon2 100))
  (Variables|Default|SetCurrentMagWeapon2 _output_get_2)
  (Variables|Default|SetRemainingAmmoWeapon2 300)
  (CallFunction|WeaponSelect))

(event Collision|EventActorBeginOverlap
  (params (OtherActor :type Actor%20Object%20Reference)))

(event EventTick
  (params (DeltaSeconds :type Float%20%28single-precision%29)))

(event Input|KeyboardEvents|3
  (params (Key :type Key%20Structure))
  (:Pressed
    (CallFunction|WeaponSelect (Utilities|KeytoInt Key))))

(event Input|KeyboardEvents|0
  (params (Key :type Key%20Structure))
  (:Pressed
    (CallFunction|WeaponSelect (Utilities|KeytoInt Key))))

(event Input|KeyboardEvents|1
  (params (Key :type Key%20Structure))
  (:Pressed
    (CallFunction|WeaponSelect (Utilities|KeytoInt Key))))

(event Input|KeyboardEvents|2
  (params (Key :type Key%20Structure))
  (:Pressed
    (CallFunction|WeaponSelect (Utilities|KeytoInt Key))))

(event Input|KeyboardEvents|Tab
  (params (Key :type Key%20Structure))
  (:Pressed
    (if (< (Variables|Default|GetWeapon%20Selection) 3)
      (CallFunction|WeaponSelect (+ (Variables|Default|GetWeapon%20Selection) 1))
      (else
        (CallFunction|WeaponSelect)))))

(event Input|KeyboardEvents|R
  (params (Key :type Key%20Structure))
  (:Pressed
    (CallFunction|Reload)))

(fn ConstructionScript)

(fn WeaponSelect
  (params (Weapon%20Type :type Integer))
  (if (and (!= (Variables|Default|GetWeapon%20Selection) 0) (== (Variables|Default|GetWeapon%20Selection) Weapon%20Type))
    (CallFunction|WeaponSelect)
    (else
      (CallFunction|ResetWeapons)
      (Development|PrintString (Utilities|String|Append (Utilities|String|Append "Weapon " (Utilities|String|ToString(Integer) Weapon%20Type)) " Selected!"))
      (bind _output_get (Variables|Default|SetWeapon%20Selection Weapon%20Type))
      (bind _asgi_cube_game_instance (Utilities|Casting|CastToGI_CubeGameInstance (Game|GetGameInstance)))
      (bind _aswbp_hud (Utilities|Casting|CastToWBP_HUD (Variables|/Game/_TheCubeAssets/Blueprints/GI_CubeGameInstance.GI_CubeGameInstance_C|GetHUD%20Widget _asgi_cube_game_instance)))
      (Default|SetWeapon _aswbp_hud _output_get)
      (switch int _output_get
        (:Default
          (CallFunction|ResetWeapons :!label _label))
        (:0
          (goto _label))
        (:1
          (bind _asbp_first_person_character (Utilities|Casting|CastToBP_FirstPersonCharacter (Game|Player|GetPlayerPawn 0)))
          (if (not (Variables|/Game/_TheCubeAssets/Blueprints/Player/Blueprints/BP_FirstPersonCharacter.BP_FirstPersonCharacter_C|GetbHasRifle _asbp_first_person_character))
            (AddComponent|AddBPWeaponComponent _asbp_first_person_character false)
            (CallFunction|UpdateWeapon1Text)))
        (:2
          (bind _asbp_first_person_character_2 (Utilities|Casting|CastToBP_FirstPersonCharacter (Game|Player|GetPlayerPawn 0)))
          (if (not (Variables|/Game/_TheCubeAssets/Blueprints/Player/Blueprints/BP_FirstPersonCharacter.BP_FirstPersonCharacter_C|GetbHasMiniGun _asbp_first_person_character_2))
            (Development|PrintString "Minigun Spawned")
            (bind _returnvalue (Game|SpawnActorfromClass "/Game/_TheCubeAssets/Blueprints/Player/MiniGunWeapon/Minigun.Minigun_C" (Math|Transform|MakeTransform "10.000000,20.000000,25.000000") "Undefined" "MultiplyWithRoot" 0 0))
            (Transformation|AttachActorToActor _returnvalue _asbp_first_person_character_2 "None" "KeepRelative" "KeepRelative" "KeepRelative" true)
            (CallFunction|UpdateWeapon2Text)))
        (:3
          (goto _label))))))

(fn AddAmmoWeapon1
  (params (Ammo%20To%20Add :type Integer))
  (Variables|Default|SetRemainingAmmoWeapon1 (+ Ammo%20To%20Add (Variables|Default|GetRemainingAmmoWeapon1)))
  (if (== (Variables|Default|GetWeapon%20Selection) 1)
    (CallFunction|UpdateWeapon1Text)))

(fn Reload
  (bind _magsizeweapon1 (Variables|Default|GetMagSizeWeapon1))
  (bind _magsizeweapon2 (Variables|Default|GetMagSizeWeapon2))
  (switch int (Variables|Default|GetWeapon%20Selection)
    (:Default
      (return))
    (:0
      (return))
    (:1
      ;[1 1 1] Weapon 1
      (bind _asbp_first_person_character (Utilities|Casting|CastToBP_FirstPersonCharacter (Game|Player|GetPlayerPawn 0)))
      (if (and (!= (Variables|Default|GetCurrentMagWeapon1) (Variables|Default|GetMagSizeWeapon1)) (> (Variables|Default|GetRemainingAmmoWeapon1) 0))
        (Default|ReloadSound (Variables|/Game/_TheCubeAssets/Blueprints/Player/Blueprints/BP_FirstPersonCharacter.BP_FirstPersonCharacter_C|GetWeapon _asbp_first_person_character))
        (Variables|Default|SetRemainingAmmoWeapon1 (+ (Variables|Default|GetRemainingAmmoWeapon1) (Variables|Default|GetCurrentMagWeapon1)))
        (if (>= (Variables|Default|GetRemainingAmmoWeapon1) (Variables|Default|GetMagSizeWeapon1))
          (Variables|Default|SetRemainingAmmoWeapon1 (- (Variables|Default|GetRemainingAmmoWeapon1) _magsizeweapon1))
          (Variables|Default|SetCurrentMagWeapon1 _magsizeweapon1)
          (else
            (Variables|Default|SetCurrentMagWeapon1 (Variables|Default|GetRemainingAmmoWeapon1))
            (Variables|Default|SetRemainingAmmoWeapon1 0)))
        (CallFunction|UpdateWeapon1Text)
        (return)))
    (:2
      ;[1 1 1] Weapon 2
      (bind _returnvalue (Actor|GetActorOfClass "/Game/_TheCubeAssets/Blueprints/Player/MiniGunWeapon/Minigun.Minigun_C"))
      (if (and (!= (Variables|Default|GetCurrentMagWeapon2) (Variables|Default|GetMagSizeWeapon2)) (> (Variables|Default|GetRemainingAmmoWeapon2) 0))
        (Default|ReloadSound _returnvalue)
        (Variables|Default|SetRemainingAmmoWeapon2 (+ (Variables|Default|GetRemainingAmmoWeapon2) (Variables|Default|GetCurrentMagWeapon2)))
        (if (>= (Variables|Default|GetRemainingAmmoWeapon2) (Variables|Default|GetMagSizeWeapon2))
          (Variables|Default|SetRemainingAmmoWeapon2 (- (Variables|Default|GetRemainingAmmoWeapon2) _magsizeweapon2))
          (Variables|Default|SetCurrentMagWeapon2 _magsizeweapon2)
          (else
            (Variables|Default|SetCurrentMagWeapon2 (Variables|Default|GetRemainingAmmoWeapon2))
            (Variables|Default|SetRemainingAmmoWeapon2 0)))
        (CallFunction|UpdateWeapon2Text)
        (return)))
    (:3
      (return))))

(fn UpdateWeapon1Text
  (bind _asgi_cube_game_instance (Utilities|Casting|CastToGI_CubeGameInstance (Game|GetGameInstance)))
  (bind _aswbp_hud (Utilities|Casting|CastToWBP_HUD (Variables|/Game/_TheCubeAssets/Blueprints/GI_CubeGameInstance.GI_CubeGameInstance_C|GetHUD%20Widget _asgi_cube_game_instance)))
  (Default|UpdateText _aswbp_hud (Utilities|String|Append "Gun  " (Utilities|String|Append (Utilities|String|Append (Utilities|String|ToString(Integer) (Variables|Default|GetCurrentMagWeapon1)) "/") (Utilities|String|ToString(Integer) (Variables|Default|GetRemainingAmmoWeapon1))))))

(fn ResetWeapons
  (bind _returnvalue (Game|GetPlayerController 0))
  (bind _returnvalue_2 (Game|GetPlayerController 0))
  (bind _returnvalue_3 (PlayerController|LocalPlayerSubsystems|GetEnhancedInputLocalPlayerSubsystem _returnvalue))
  (bind _returnvalue_4 (PlayerController|LocalPlayerSubsystems|GetEnhancedInputLocalPlayerSubsystem _returnvalue_2))
  (bind _returnvalue_5 (Actor|GetActorOfClass "/Game/_TheCubeAssets/Blueprints/Player/MiniGunWeapon/Minigun.Minigun_C"))
  (if (Utilities|IsValid _returnvalue_3)
    (Input|RemoveMappingContext _returnvalue_3 "/Game/_TheCubeAssets/Blueprints/Player/MiniGunWeapon/IMC_Minigun.IMC_Minigun" "(bIgnoreAllPressedKeysUntilRelease=True,bForceImmediately=False,bNotifyUserSettings=False)")
    (if (Utilities|IsValid _returnvalue_5)
      (Actor|DestroyActor _returnvalue_5))
    (bind _asbp_first_person_character (Utilities|Casting|CastToBP_FirstPersonCharacter (Game|Player|GetPlayerPawn 0)))
    (Variables|/Game/_TheCubeAssets/Blueprints/Player/Blueprints/BP_FirstPersonCharacter.BP_FirstPersonCharacter_C|SetbHasMiniGun _asbp_first_person_character false)
    (if (Utilities|IsValid (Variables|/Game/_TheCubeAssets/Blueprints/Player/Blueprints/BP_FirstPersonCharacter.BP_FirstPersonCharacter_C|GetWeapon _asbp_first_person_character))
      (if (not (Class|ActorComponent|IsBeingDestroyed (Variables|/Game/_TheCubeAssets/Blueprints/Player/Blueprints/BP_FirstPersonCharacter.BP_FirstPersonCharacter_C|GetWeapon _asbp_first_person_character)))
        (Default|DestroyThis (Variables|/Game/_TheCubeAssets/Blueprints/Player/Blueprints/BP_FirstPersonCharacter.BP_FirstPersonCharacter_C|GetWeapon _asbp_first_person_character)))
      (Variables|/Game/_TheCubeAssets/Blueprints/Player/Blueprints/BP_FirstPersonCharacter.BP_FirstPersonCharacter_C|SetbHasRifle _asbp_first_person_character false)
      (if (Utilities|IsValid _returnvalue_4)
        (Input|RemoveMappingContext _returnvalue_4 "/Game/_TheCubeAssets/Blueprints/Player/Input/IMC_Weapons.IMC_Weapons" "(bIgnoreAllPressedKeysUntilRelease=True,bForceImmediately=False,bNotifyUserSettings=False)")
        (Variables|/Game/_TheCubeAssets/Blueprints/Player/Blueprints/BP_FirstPersonCharacter.BP_FirstPersonCharacter_C|SetWeapon _asbp_first_person_character (Variables|Default|GetNULL%20WEAPON))))))

(fn AddAmmoWeapon2
  (params (Ammo%20To%20Add :type Integer))
  (Variables|Default|SetRemainingAmmoWeapon2 (+ Ammo%20To%20Add (Variables|Default|GetRemainingAmmoWeapon2)))
  (if (== (Variables|Default|GetWeapon%20Selection) 2)
    (CallFunction|UpdateWeapon2Text)))

(fn UpdateWeapon2Text
  (bind _asgi_cube_game_instance (Utilities|Casting|CastToGI_CubeGameInstance (Game|GetGameInstance)))
  (bind _aswbp_hud (Utilities|Casting|CastToWBP_HUD (Variables|/Game/_TheCubeAssets/Blueprints/GI_CubeGameInstance.GI_CubeGameInstance_C|GetHUD%20Widget _asgi_cube_game_instance)))
  (Default|UpdateText _aswbp_hud (Utilities|String|Append "Minigun  " (Utilities|String|Append (Utilities|String|Append (Utilities|String|ToString(Integer) (Variables|Default|GetCurrentMagWeapon2)) "/") (Utilities|String|ToString(Integer) (Variables|Default|GetRemainingAmmoWeapon2))))))