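; Level manager for a cube world that finds or spawns six I_Level actors, attaches one per face, and rotates to switch between them.
; SwitchSide, called by NextLevel or debug numpad keys, ends all levels and sets the target rotation.
; Tick glides the player to the centre, lerps the cube's rotation while holding them there, then begins the chosen level.
; ClearBlankHolder recursively destroys leftover actors attached to the Blank holder.
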(event EventBeginPlay
  (CallFunction|Spawn-Levels)
  (Variables|Default|SetRotationTriggered false)
  (Variables|Default|SetPlayerLifted false)
  ;[1 0 0.8051] DEBUG ONLY
  (Variables|Default|SetDEBUG false)
  (Variables|Default|SetLevel%20To%20Play -1))

(event Collision|EventActorBeginOverlap
  (params (OtherActor :type Actor%20Object%20Reference)))

(event EventTick
  (params (DeltaSeconds :type Float%20%28single-precision%29))
  (CallFunction|RotationLogic DeltaSeconds))

(event Input|KeyboardEvents|DebugKeyNumPadZero
  (params (Key :type Key%20Structure :default "None") (ActionValue :type Input%20Action%20Value%20Structure))
  ;[1 0 0.8051] DEBUG
  (:Pressed
    (Utilities|IsDebug
      (:OUT
        (CallFunction|SwitchSide)))))

(event Input|KeyboardEvents|DebugKeyNumPadOne
  (params (Key :type Key%20Structure :default "None") (ActionValue :type Input%20Action%20Value%20Structure))
  ;[1 0 0.8051] DEBUG
  (:Pressed
    (Utilities|IsDebug
      (:OUT
        (CallFunction|SwitchSide 1)))))

(event Input|KeyboardEvents|DebugKeyNumPadTwo
  (params (Key :type Key%20Structure :default "None") (ActionValue :type Input%20Action%20Value%20Structure))
  ;[1 0 0.8051] DEBUG
  (:Pressed
    (Utilities|IsDebug
      (:OUT
        (CallFunction|SwitchSide 2)))))

(event Input|KeyboardEvents|DebugKeyNumPadThree
  (params (Key :type Key%20Structure :default "None") (ActionValue :type Input%20Action%20Value%20Structure))
  ;[1 0 0.8051] DEBUG
  (:Pressed
    (Utilities|IsDebug
      (:OUT
        (CallFunction|SwitchSide 3)))))

(event Input|KeyboardEvents|DebugKeyNumPadFour
  (params (Key :type Key%20Structure :default "None") (ActionValue :type Input%20Action%20Value%20Structure))
  ;[1 0 0.8051] DEBUG
  (:Pressed
    (Utilities|IsDebug
      (:OUT
        (CallFunction|SwitchSide 4)))))

(event Input|KeyboardEvents|DebugKeyNumPadFive
  (params (Key :type Key%20Structure :default "None") (ActionValue :type Input%20Action%20Value%20Structure))
  ;[1 0 0.8051] DEBUG
  (:Pressed
    (Utilities|IsDebug
      (:OUT
        (CallFunction|SwitchSide 5)))))

(fn ConstructionScript)

(fn SwitchSide
  (params (Side :type Integer))
  (for _array_element (Variables|Default|GetLevelsInterface)
    (Default|LevelEnded _array_element))
  (bind _output_get (Variables|Default|SetLevel%20To%20Play Side))
  ;[1 0 0.006721] Check is valid value
  (if (and (>= Side 0) (<= Side 5))
    (switch int _output_get
      (:Default
        ;[1 0 0.8051] DEBUG
        (if (Variables|Default|GetDEBUG) :!label _label
          (Development|PrintString "ERROR: Invalid side (int) to switch to..." true true "(R=1.000000,G=0.000000,B=0.000000,A=1.000000)")))
      (:0
        (Variables|Default|SetTarget%20Rotation "0, 0, 0")
        (Variables|Default|SetRotationTriggered true :!label _label_2)
        ;[1 0 0.8051] DEBUG
        (if (Variables|Default|GetDEBUG)
          (Development|PrintString (Utilities|String|Append "Rotating cube to " (Utilities|String|ToString(Rotator) (Variables|Default|GetTarget%20Rotation))) true true "(R=0.656360,G=0.000000,B=1.000000,A=1.000000)")))
      (:1
        (Variables|Default|SetTarget%20Rotation "0.000000,0.000000,90.000000")
        (goto _label_2))
      (:2
        (Variables|Default|SetTarget%20Rotation "-90.000000,0.000000,0.000000")
        (goto _label_2))
      (:3
        (Variables|Default|SetTarget%20Rotation "90.000000,0.000000,0.000000")
        (goto _label_2))
      (:4
        (Variables|Default|SetTarget%20Rotation "0.000000,0.000000,-90.000000")
        (goto _label_2))
      (:5
        (Variables|Default|SetTarget%20Rotation "0.000000,180.000000,180.000000")
        (goto _label_2)))
    (else
      (goto _label))))

(fn CheckifAlmostSame
  (params (R1 :type Rotator) (R2 :type Rotator) (Tollerance :type Float%20%28double-precision%29))
  (return (Utilities|Operators|EqualEqual R1 R2 Tollerance)))

(fn CheckifPlayerLifted
  (params (R1 :type Vector) (R2 :type Vector) (Tollerance :type Float%20%28double-precision%29))
  (return (Utilities|Operators|EqualEqual R1 R2 Tollerance)))

(fn ClearBlankHolder
  ;[1 0.02501 0] Deletes any temporary assets spawns from previously level attached to blank holder
  (bind _returnvalue (Actor|GetActorOfClass "/Game/_TheCubeAssets/Blueprints/Levels/Blank.Blank_C"))
  ;;[0.9632 0 1] ------------------------BUG FIXED DIRTY HERE ----------------------------
  (for _array_element (Actor|GetAttachedActors _returnvalue true true)
    (if (not (== _returnvalue _array_element))
      (Actor|DestroyActor _array_element)))
  (if (== (Utilities|Array|Length (Actor|GetAttachedActors _returnvalue true true)) 0)
    (return)
    (else
      (CallFunction|ClearBlankHolder))))

(fn Spawn-Levels
  (bind _sidetransforms (Variables|Default|GetSideTransforms))
  ;[0 0 0] Initilize
  ;;[0.1354 1 0] 100 * scale of base * 0.5
  (Variables|Default|SetLevel%20Depth 2e+03)
  (Utilities|Array|Add _sidetransforms (Math|Transform|MakeTransform (Math|Vector|MakeVector 0.0 0.0 (* (Variables|Default|GetLevel%20Depth) -1.0))))
  (Utilities|Array|Add _sidetransforms (Math|Transform|MakeTransform (Math|Vector|MakeVector 0.0 (Variables|Default|GetLevel%20Depth) 0.0) "0.000000,0.000000,90.000000"))
  (Utilities|Array|Add _sidetransforms (Math|Transform|MakeTransform (Math|Vector|MakeVector (Variables|Default|GetLevel%20Depth) 0.0 0.0) "90.000000,0.000000,0.000000"))
  (Utilities|Array|Add _sidetransforms (Math|Transform|MakeTransform (Math|Vector|MakeVector (* (Variables|Default|GetLevel%20Depth) -1.0) 0.0 0.0) "270.000000,0.000000,0.000000"))
  (Utilities|Array|Add _sidetransforms (Math|Transform|MakeTransform (Math|Vector|MakeVector 0.0 (* (Variables|Default|GetLevel%20Depth) -1.0) 0.0) "0.000000,0.000000,270.000000"))
  (Utilities|Array|Add _sidetransforms (Math|Transform|MakeTransform (Math|Vector|MakeVector 0.0 0.0 (Variables|Default|GetLevel%20Depth)) "0.000000,0.000000,180.000000"))
  ;;[0.9964 1 0.5167] Try Create Levels
  (bind _returnvalue (Actor|GetActorOfClass "/Game/_TheCubeAssets/Blueprints/Levels/L_0_Level-Maze.L_0_Level-Maze_C"))
  (if (Utilities|IsValid _returnvalue)
    (bind _asi_level (Utilities|Casting|CastToI_Level _returnvalue))
    (Utilities|Array|Add (Variables|Default|GetLevelsInterface) _asi_level)
    (else
      (bind _returnvalue_2 (Game|SpawnActorfromClass "/Game/_TheCubeAssets/Blueprints/Levels/L_0_Level-Maze.L_0_Level-Maze_C" (Variables|Default|GetTransformBLANK) "Undefined" "MultiplyWithRoot" 0 0))
      (bind _asi_level_2 (Utilities|Casting|CastToI_Level _returnvalue_2))
      (Utilities|Array|Add (Variables|Default|GetLevelsInterface) _asi_level_2)))
  (bind _returnvalue_3 (Actor|GetActorOfClass "/Game/_TheCubeAssets/Blueprints/Levels/L_1_Level-Waves.L_1_Level-Waves_C"))
  (if (Utilities|IsValid _returnvalue_3)
    (bind _asi_level_3 (Utilities|Casting|CastToI_Level _returnvalue_3))
    (Utilities|Array|Add (Variables|Default|GetLevelsInterface) _asi_level_3)
    (else
      (bind _returnvalue_4 (Game|SpawnActorfromClass "/Game/_TheCubeAssets/Blueprints/Levels/L_1_Level-Waves.L_1_Level-Waves_C" (Variables|Default|GetTransformBLANK) "Undefined" "MultiplyWithRoot" 0 0))
      (bind _asi_level_4 (Utilities|Casting|CastToI_Level _returnvalue_4))
      (Utilities|Array|Add (Variables|Default|GetLevelsInterface) _asi_level_4)))
  (bind _returnvalue_5 (Actor|GetActorOfClass "/Game/_TheCubeAssets/Blueprints/Levels/L_2_Level-Parkour.L_2_Level-Parkour_C"))
  (if (Utilities|IsValid _returnvalue_5)
    (bind _asi_level_5 (Utilities|Casting|CastToI_Level _returnvalue_5))
    (Utilities|Array|Add (Variables|Default|GetLevelsInterface) _asi_level_5)
    (else
      (bind _returnvalue_6 (Game|SpawnActorfromClass "/Game/_TheCubeAssets/Blueprints/Levels/L_2_Level-Parkour.L_2_Level-Parkour_C" (Variables|Default|GetTransformBLANK) "Undefined" "MultiplyWithRoot" 0 0))
      (bind _asi_level_6 (Utilities|Casting|CastToI_Level _returnvalue_6))
      (Utilities|Array|Add (Variables|Default|GetLevelsInterface) _asi_level_6)))
  (bind _returnvalue_7 (Actor|GetActorOfClass "/Game/_TheCubeAssets/Blueprints/Levels/L_3_Level-Cubes.L_3_Level-Cubes_C"))
  (if (Utilities|IsValid _returnvalue_7)
    (bind _asi_level_7 (Utilities|Casting|CastToI_Level _returnvalue_7))
    (Utilities|Array|Add (Variables|Default|GetLevelsInterface) _asi_level_7)
    (else
      (bind _returnvalue_8 (Game|SpawnActorfromClass "/Game/_TheCubeAssets/Blueprints/Levels/L_3_Level-Cubes.L_3_Level-Cubes_C" (Variables|Default|GetTransformBLANK) "Undefined" "MultiplyWithRoot" 0 0))
      (bind _asi_level_8 (Utilities|Casting|CastToI_Level _returnvalue_8))
      (Utilities|Array|Add (Variables|Default|GetLevelsInterface) _asi_level_8)))
  (bind _returnvalue_9 (Actor|GetActorOfClass "/Game/_TheCubeAssets/Blueprints/Levels/L_4_Level-Problem.L_4_Level-Problem_C"))
  (if (Utilities|IsValid _returnvalue_9)
    (bind _asi_level_9 (Utilities|Casting|CastToI_Level _returnvalue_9))
    (Utilities|Array|Add (Variables|Default|GetLevelsInterface) _asi_level_9)
    (else
      (bind _returnvalue_10 (Game|SpawnActorfromClass "/Game/_TheCubeAssets/Blueprints/Levels/L_4_Level-Problem.L_4_Level-Problem_C" (Variables|Default|GetTransformBLANK) "Undefined" "MultiplyWithRoot" 0 0))
      (bind _asi_level_10 (Utilities|Casting|CastToI_Level _returnvalue_10))
      (Utilities|Array|Add (Variables|Default|GetLevelsInterface) _asi_level_10)))
  (bind _returnvalue_11 (Actor|GetActorOfClass "/Game/_TheCubeAssets/Blueprints/Levels/L_5_Level-Boss.L_5_Level-Boss_C"))
  (if (Utilities|IsValid _returnvalue_11)
    (bind _asi_level_11 (Utilities|Casting|CastToI_Level _returnvalue_11))
    (Utilities|Array|Add (Variables|Default|GetLevelsInterface) _asi_level_11)
    (else
      (bind _returnvalue_12 (Game|SpawnActorfromClass "/Game/_TheCubeAssets/Blueprints/Levels/L_5_Level-Boss.L_5_Level-Boss_C" (Variables|Default|GetTransformBLANK) "Undefined" "MultiplyWithRoot" 0 0))
      (bind _asi_level_12 (Utilities|Casting|CastToI_Level _returnvalue_12))
      (Utilities|Array|Add (Variables|Default|GetLevelsInterface) _asi_level_12)))
  ;[0 0.05366 1] Move all transforms and Deactive
  (for (_array_element _array_index) (Variables|Default|GetLevelsInterface)
    (if (Variables|Default|GetDEBUG)
      ;;[1 0 0.8051] DEBUG
      (Development|PrintString (Utilities|String|Append (Utilities|String|Append (Utilities|String|Append "Initialized Level " (Utilities|String|ToString(Integer) _array_index)) " @ transform ") (Utilities|String|ToString(Transform) (Utilities|Array|Get(acopy) (Variables|Default|GetSideTransforms) _array_index))) true true "(R=0.000000,G=1.000000,B=0.019042,A=1.000000)"))
    (Default|SpawnLevel _array_element (Utilities|Array|Get(acopy) (Variables|Default|GetSideTransforms) _array_index))
    (bind _asactor (Utilities|Casting|CastToActor (Utilities|ToObject(Interface) _array_element))
      (:then
        (Transformation|AttachActorToActor _asactor self "None" "KeepRelative" "KeepRelative" "KeepRelative" true))
      (:CastFailed
        (Development|PrintString "Error: Unable to cast target to actor #876" true true "(R=1.000000,G=0.000000,B=0.000000,A=1.000000)")))))

(fn RotationLogic
  (params (DeltaTime :type Float%20%28double-precision%29))
  (bind _returnvalue (Game|GetPlayerCharacter 0))
  (bind _returnvalue_2 (Game|GetPlayerCharacter 0))
  (bind _returnvalue_3 (Transformation|GetActorLocation _returnvalue_2))
  (Transformation|SetWorldLocation (Variables|Default|GetDefaultSceneRoot self) "0, 0, 0" false false)
  ;[0 1 0.8959] ROTATE THE CUBE!!!
  (if (Variables|Default|GetRotationTriggered)
    (if (Variables|Default|GetPlayerLifted)
      (Transformation|SetActorLocation _returnvalue_3 false true)
      (bind _minimaldifference (CallFunction|CheckifAlmostSame (Transformation|GetActorRotation) (Variables|Default|GetTarget%20Rotation) 0.5))
      (if _minimaldifference
        (Variables|Default|SetPlayerLifted false)
        (Transformation|SetActorLocation _returnvalue "0, 0, 0" false false)
        (Variables|Default|SetRotationTriggered false)
        (Default|LevelBegin (Utilities|Array|Get(acopy) (Variables|Default|GetLevelsInterface) (Variables|Default|GetLevel%20To%20Play)))
        (Transformation|SetActorRotation (Variables|Default|GetTarget%20Rotation) true :!label _label)
        (return)
        (else
          (Transformation|SetActorRotation (Math|Rotator|Lerp(Rotator) (Transformation|GetActorRotation) (Variables|Default|GetTarget%20Rotation) (* DeltaTime 1.25)) true)
          (Transformation|SetActorLocation _returnvalue "0, 0, 0" false false)
          (return)))
      (else
        (Pawn|Components|CharacterMovement|SetMovementMode (Variables|/Script/Engine.Character|GetCharacterMovement (Game|GetPlayerCharacter 0)) "MOVE_None" 0)
        (Transformation|SetActorLocation _returnvalue_2 (Math|Vector|Lerp(Vector) (Transformation|GetActorLocation _returnvalue_2) "0.000000,0.000000,10.000000" (* DeltaTime 1.0)) false true)
        (if (< (Math|Vector|Distance(Vector) _returnvalue_3 "0, 0, 0") 1e+01)
          (Pawn|Components|CharacterMovement|SetMovementMode (Variables|/Script/Engine.Character|GetCharacterMovement _returnvalue_2) "MOVE_Falling" 0)
          (Variables|Default|SetPlayerLifted true))))
    (else
      (goto _label))))

(fn NextLevel
  (CallFunction|SwitchSide (+ (Variables|Default|GetLevel%20To%20Play) 1)))