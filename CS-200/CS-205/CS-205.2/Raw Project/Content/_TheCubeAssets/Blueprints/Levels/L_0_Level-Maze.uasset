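; Maze level actor for the cube game, running the level from begin to end and updating the HUD objective.
; On begin it spawns ten ranged enemies at random locations borrowed from L_1_LevelWaves, attached to the Blank actor.
; While in progress, Tick spawns the MazeObject if missing and lerps it upward to raise the walls.
; Tick also polls for BP_Key actors and calls LevelManager's NextLevel when none remain.
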(event EventBeginPlay
  (Variables|Default|SetLevel%20Number 0))

(event Collision|EventActorBeginOverlap
  (params (OtherActor :type Actor%20Object%20Reference)))

(event EventTick
  (params (DeltaSeconds :type Float%20%28single-precision%29))
  (if (Variables|Default|GetLevel%20In%20Progress)
    (CallFunction|RaiseBarriers DeltaSeconds)
    (CallFunction|CheckKeys)))

(event EventSpawnLevel
  (params (Transform :type Transform))
  (Transformation|SetActorTransform Transform false true)
  (Variables|Default|SetLevel%20In%20Progress false))

(event EventLevelBegin
  (Variables|Default|SetLevel%20In%20Progress true)
  (Development|PrintString (Utilities|String|Append (Utilities|String|Append "Level " (Utilities|String|ToString(Integer) (Variables|Default|GetLevel%20Number))) " started!"))
  ;[0 0.9639 1] Show Objective
  (bind _asgi_cube_game_instance (Utilities|Casting|CastToGI_CubeGameInstance (Game|GetGameInstance)))
  (bind _aswbp_hud (Utilities|Casting|CastToWBP_HUD (Variables|/Game/_TheCubeAssets/Blueprints/GI_CubeGameInstance.GI_CubeGameInstance_C|GetHUD%20Widget _asgi_cube_game_instance)))
  (Default|ShowObjective _aswbp_hud (+ (Variables|Default|GetLevel%20Number) 1))
  ;[0.141 0 1] Level start
  (Variables|Default|SetRaise true)
  (Variables|Default|SetRaiseComplete false)
  (bind _returnvalue (Actor|GetActorOfClass "/Game/_TheCubeAssets/Blueprints/Levels/L_1_Level-Waves.L_1_Level-Waves_C"))
  (for _index (range 0 9)
    (bind _random (Default|RandomLocation _returnvalue))
    (bind _returnvalue_2 (Actor|GetActorOfClass "/Game/_TheCubeAssets/Blueprints/Levels/Blank.Blank_C"))
    (bind _returnvalue_3 (Game|SpawnActorfromClass "/Game/_TheCubeAssets/Blueprints/Enemies/Ranged_Enemy.Ranged_Enemy_C" _random "AdjustIfPossibleButAlwaysSpawn" "MultiplyWithRoot" 0 0))
    (Transformation|AttachActorToActor _returnvalue_3 _returnvalue_2 "None" "KeepRelative" "KeepRelative" "KeepRelative" true)))

(fn ConstructionScript)

(fn RaiseBarriers
  (params (DT :type Float%20%28double-precision%29))
  ;[1 0.2339 0] Raises the Maze Walls
  (if (Variables|Default|GetRaise)
    (if (Variables|Default|GetRaiseComplete)
      (return)
      (else
        (bind _returnvalue (Actor|GetActorOfClass "/Game/_TheCubeAssets/Blueprints/Levels/L_0-Maze/MazeObject.MazeObject_C"))
        (if (Utilities|IsValid _returnvalue)
          (Transformation|SetActorLocation _returnvalue (Math|Vector|Lerp(Vector) (Transformation|GetActorLocation _returnvalue) "0.000000,0.000000,-1950.000000" DT) false true)
          (if (< (Math|Vector|Distance(Vector) "0.000000,0.000000,-2000.000000" (Math|Vector|Lerp(Vector) (Transformation|GetActorLocation _returnvalue) "0.000000,0.000000,-1950.000000" DT)) 5.0)
            (Variables|Default|SetRaiseComplete true))
          (else
            (bind _returnvalue_2 (Game|SpawnActorfromClass "/Game/_TheCubeAssets/Blueprints/Levels/L_0-Maze/MazeObject.MazeObject_C" (Math|Transform|MakeTransform "0.000000,0.000000,-2300.000000") "AlwaysSpawn" "MultiplyWithRoot" 0 0))
            (bind _returnvalue_3 (Actor|GetActorOfClass "/Game/_TheCubeAssets/Blueprints/Levels/Blank.Blank_C"))
            (Transformation|AttachActorToActor _returnvalue_2 _returnvalue_3 "None" "KeepRelative" "KeepRelative" "KeepRelative" false)))))
    (else
      (return))))

(fn CheckKeys
  (bind _outactors (Actor|GetAllActorsOfClass "/Game/_TheCubeAssets/Blueprints/Items/BP_Key.BP_Key_C"))
  (if (== (Utilities|Array|Length _outactors) 0)
    (bind _returnvalue (Actor|GetActorOfClass "/Game/_TheCubeAssets/Blueprints/LevelManager.LevelManager_C"))
    (Default|NextLevel _returnvalue)))

(fn GetLevelNumber
  (return (Variables|Default|GetLevel%20Number)))

(fn LevelEnded
  (if (Variables|Default|GetLevel%20In%20Progress)
    (Development|PrintString (Utilities|String|Append (Utilities|String|Append "Level " (Utilities|String|ToString(Integer) (Variables|Default|GetLevel%20Number))) " ended!"))
    ;[1 0.796 0] Complete Objective
    (bind _asgi_cube_game_instance (Utilities|Casting|CastToGI_CubeGameInstance (Game|GetGameInstance)))
    (bind _aswbp_hud (Utilities|Casting|CastToWBP_HUD (Variables|/Game/_TheCubeAssets/Blueprints/GI_CubeGameInstance.GI_CubeGameInstance_C|GetHUD%20Widget _asgi_cube_game_instance)))
    (Default|CompleteObjective _aswbp_hud (+ 0 1)))
  (Variables|Default|SetLevel%20In%20Progress false)
  (return))