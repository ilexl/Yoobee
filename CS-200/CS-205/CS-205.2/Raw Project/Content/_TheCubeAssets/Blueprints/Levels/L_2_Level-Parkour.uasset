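; Level 2 parkour actor: a rising-lava arena with breakable platforms and flying ranged enemies, reporting its objective to the HUD.
; Flag-driven Tick stages lerp four glass walls up, spawn lava, then raise it until a target height triggers LevelManager's NextLevel.
; During the rise, platforms ride the lava and replenish at random positions, while enemy waves spawn periodically.
; Spawns attach to a Blank holder, which LevelEnded clears through LevelManager.
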(event EventBeginPlay
  (Variables|Default|SetLevel%20Number 2))

(event Collision|EventActorBeginOverlap
  (params (OtherActor :type Actor%20Object%20Reference)))

(event EventTick
  (params (DeltaSeconds :type Float%20%28single-precision%29))
  ;[1 1 1] Loop Logic
  (if (Variables|Default|GetLevel%20In%20Progress)
    (if (Variables|Default|GetToMoveGlassUp)
      (CallFunction|MovePlatformsUp DeltaSeconds))
    (if (Variables|Default|GetSpawnLava)
      (CallFunction|CreateLava))
    (if (Variables|Default|GetRISE)
      (bind _z (CallFunction|RiseLogic DeltaSeconds))
      (CallFunction|SpawnEnemiesOverTime DeltaSeconds _z))))

(event EventLevelBegin
  ;[1 0.9369 0] Setup
  (Variables|Default|SetLevel%20In%20Progress true)
  (Development|PrintString (Utilities|String|Append (Utilities|String|Append "Level " (Utilities|String|ToString(Integer) (Variables|Default|GetLevel%20Number))) " started!"))
  ;[0 1 0.3254] Show Objective
  (bind _asgi_cube_game_instance (Utilities|Casting|CastToGI_CubeGameInstance (Game|GetGameInstance)))
  (bind _aswbp_hud (Utilities|Casting|CastToWBP_HUD (Variables|/Game/_TheCubeAssets/Blueprints/GI_CubeGameInstance.GI_CubeGameInstance_C|GetHUD%20Widget _asgi_cube_game_instance)))
  (Default|ShowObjective _aswbp_hud (+ (Variables|Default|GetLevel%20Number) 1))
  (CallFunction|GlassPanelsStart))

(event EventSpawnLevel
  (params (Transform :type Transform))
  (Transformation|SetActorTransform Transform false true)
  (Variables|Default|SetLevel%20In%20Progress false))

(fn ConstructionScript)

(fn RiseLogic
  (params (DT :type Float%20%28double-precision%29))
  (bind _returnvalue (Transformation|GetActorTransform))
  (bind (_location _rotation _scale) (Math|Transform|BreakTransform _returnvalue))
  (bind (_x _y) (Math|Vector|BreakVector _location))
  ;[1 0.6854 0] Raises objects up as if the lava is rising
  (bind _returnvalue_2 (Actor|GetActorOfClass "/Game/_TheCubeAssets/Blueprints/Levels/L_2-Parkour/Lava.Lava_C"))
  (Transformation|SetActorTransform _returnvalue_2 (Math|Transform|MakeTransform (Math|Vector|MakeVector _x _y (+ (.Z (Math|Vector|BreakVector (.Location (Math|Transform|BreakTransform (Transformation|GetActorTransform _returnvalue_2))))) (* DT (Variables|Default|GetRiseRate)))) _rotation _scale))
  (Development|PrintString (Utilities|String|ToString(Float) (+ (.Z (Math|Vector|BreakVector (.Location (Math|Transform|BreakTransform (Transformation|GetActorTransform _returnvalue_2))))) (* DT (Variables|Default|GetRiseRate)))))
  (if (< (Math|Float|Absolute(Float) (- (+ (.Z (Math|Vector|BreakVector (.Location (Math|Transform|BreakTransform (Transformation|GetActorTransform _returnvalue_2))))) (* DT (Variables|Default|GetRiseRate))) -2.5e+02)) 1.0)
    (bind _returnvalue_3 (Actor|GetActorOfClass "/Game/_TheCubeAssets/Blueprints/LevelManager.LevelManager_C"))
    (Default|NextLevel _returnvalue_3)
    (else
      (bind _outactors (Actor|GetAllActorsOfClass "/Game/_TheCubeAssets/Blueprints/Levels/L_2-Parkour/BreakablePlatform.BreakablePlatform_C"))
      (for (_array_element _array_index) _outactors
        (Transformation|SetActorTransform _array_element (Math|Transform|MakeTransform (Math|Vector|MakeVector (.X (Math|Vector|BreakVector (.Location (Math|Transform|BreakTransform (Transformation|GetActorTransform _array_element))))) (.Y (Math|Vector|BreakVector (.Location (Math|Transform|BreakTransform (Transformation|GetActorTransform _array_element))))) (+ (+ (.Z (Math|Vector|BreakVector (.Location (Math|Transform|BreakTransform (Transformation|GetActorTransform _returnvalue_2))))) (* DT (Variables|Default|GetRiseRate))) (* (Math|Conversions|ToFloat(Integer) _array_index) 0.01))) (.Rotation (Math|Transform|BreakTransform (Transformation|GetActorTransform _array_element))) (.Scale (Math|Transform|BreakTransform (Transformation|GetActorTransform _array_element))))))
      (if (< (Utilities|Array|Length _outactors) 5)
        (bind _returnvalue_4 (Actor|GetActorOfClass "/Game/_TheCubeAssets/Blueprints/Levels/Blank.Blank_C"))
        (bind _randompos (CallFunction|GetRandomPlatformPosition (+ (+ (.Z (Math|Vector|BreakVector (.Location (Math|Transform|BreakTransform (Transformation|GetActorTransform _returnvalue_2))))) (* DT (Variables|Default|GetRiseRate))) (* (Math|Conversions|ToFloat(Integer) (Utilities|Array|Length _outactors)) 0.01))))
        (bind _returnvalue_5 (Game|SpawnActorfromClass "/Game/_TheCubeAssets/Blueprints/Levels/L_2-Parkour/BreakablePlatform.BreakablePlatform_C" (Math|Transform|MakeTransform _randompos) "AlwaysSpawn" "MultiplyWithRoot" 0 0))
        (Transformation|AttachActorToActor _returnvalue_5 _returnvalue_4 "None" "KeepWorld" "KeepWorld" "KeepWorld" false))
      (return (+ (+ (.Z (Math|Vector|BreakVector (.Location (Math|Transform|BreakTransform (Transformation|GetActorTransform _returnvalue_2))))) (* DT (Variables|Default|GetRiseRate))) (* (Math|Conversions|ToFloat(Integer) (Utilities|Array|Length _outactors)) 0.01))))))

(fn GlassPanelsStart
  ;[0.4703 0 1] Creates a glass container
  (bind _returnvalue (Actor|GetActorOfClass "/Game/_TheCubeAssets/Blueprints/Levels/Blank.Blank_C"))
  (bind _returnvalue_2 (Game|SpawnActorfromClass "/Game/_TheCubeAssets/Blueprints/Levels/L_2-Parkour/GlassWindow.GlassWindow_C" (Math|Transform|MakeTransform "0.000000,-1750.000000,-3800.000000") "AlwaysSpawn" "MultiplyWithRoot" 0 0))
  (Transformation|AttachActorToActor _returnvalue_2 _returnvalue "None" "KeepWorld" "KeepWorld" "KeepWorld" false)
  (bind _returnvalue_3 (Game|SpawnActorfromClass "/Game/_TheCubeAssets/Blueprints/Levels/L_2-Parkour/GlassWindow.GlassWindow_C" (Math|Transform|MakeTransform "0.000000,1750.000000,-3800.000000") "AlwaysSpawn" "MultiplyWithRoot" 0 0))
  (Transformation|AttachActorToActor _returnvalue_3 _returnvalue "None" "KeepWorld" "KeepWorld" "KeepWorld" false)
  (bind _returnvalue_4 (Game|SpawnActorfromClass "/Game/_TheCubeAssets/Blueprints/Levels/L_2-Parkour/GlassWindow.GlassWindow_C" (Math|Transform|MakeTransform "1750.000000,0.000000,-3800.000000" "0.000000,90.000000,0.000000") "AlwaysSpawn" "MultiplyWithRoot" 0 0))
  (Transformation|AttachActorToActor _returnvalue_4 _returnvalue "None" "KeepWorld" "KeepWorld" "KeepWorld" false)
  (bind _returnvalue_5 (Game|SpawnActorfromClass "/Game/_TheCubeAssets/Blueprints/Levels/L_2-Parkour/GlassWindow.GlassWindow_C" (Math|Transform|MakeTransform "-1750.000000,0.000000,-3800.000000" "0.000000,90.000000,0.000000") "AlwaysSpawn" "MultiplyWithRoot" 0 0))
  (Transformation|AttachActorToActor _returnvalue_5 _returnvalue "None" "KeepWorld" "KeepWorld" "KeepWorld" false)
  (Variables|Default|SetToMoveGlassUp true))

(fn CreateLava
  ;[0.6299 1 0] Creates lava
  (bind _returnvalue (Actor|GetActorOfClass "/Game/_TheCubeAssets/Blueprints/Levels/Blank.Blank_C"))
  (bind _returnvalue_2 (Game|SpawnActorfromClass "/Game/_TheCubeAssets/Blueprints/Levels/L_2-Parkour/Lava.Lava_C" (Math|Transform|MakeTransform "0.000000,0.000000,-2000.000000") "AlwaysSpawn" "MultiplyWithRoot" 0 0))
  (Transformation|AttachActorToActor _returnvalue_2 _returnvalue "None" "KeepWorld" "KeepWorld" "KeepWorld" false)
  (Variables|Default|SetSpawnLava false)
  (Variables|Default|SetRISE true))

(fn MovePlatformsUp
  (params (DT :type Float%20%28double-precision%29))
  ;[1 0 0.00858] Moves the breakable platforms up
  (bind _outactors (Actor|GetAllActorsOfClass "/Game/_TheCubeAssets/Blueprints/Levels/L_2-Parkour/GlassWindow.GlassWindow_C"))
  (for _array_element _outactors
    (Transformation|SetActorTransform _array_element (Math|Transform|Lerp(Transform) (Transformation|GetActorTransform _array_element) (Math|Transform|MakeTransform (Math|Vector|MakeVector (.X (Math|Vector|BreakVector (.Location (Math|Transform|BreakTransform (Transformation|GetActorTransform _array_element))))) (.Y (Math|Vector|BreakVector (.Location (Math|Transform|BreakTransform (Transformation|GetActorTransform _array_element))))) -2.4e+02) (.Rotation (Math|Transform|BreakTransform (Transformation|GetActorTransform _array_element))) (.Scale (Math|Transform|BreakTransform (Transformation|GetActorTransform _array_element)))) DT) false true)
    (if (<= (Math|Vector|Distance(Vector) (.Location (Math|Transform|BreakTransform (Transformation|GetActorTransform _array_element))) (Math|Vector|MakeVector (.X (Math|Vector|BreakVector (.Location (Math|Transform|BreakTransform (Transformation|GetActorTransform _array_element))))) (.Y (Math|Vector|BreakVector (.Location (Math|Transform|BreakTransform (Transformation|GetActorTransform _array_element))))) -2.4e+02)) 0.1)
      (Transformation|SetActorTransform _array_element (Math|Transform|MakeTransform (Math|Vector|MakeVector (.X (Math|Vector|BreakVector (.Location (Math|Transform|BreakTransform (Transformation|GetActorTransform _array_element))))) (.Y (Math|Vector|BreakVector (.Location (Math|Transform|BreakTransform (Transformation|GetActorTransform _array_element))))) -2.4e+02) (.Rotation (Math|Transform|BreakTransform (Transformation|GetActorTransform _array_element))) (.Scale (Math|Transform|BreakTransform (Transformation|GetActorTransform _array_element)))) false true)
      (Variables|Default|SetToMoveGlassUp false)))
  (if (not (Variables|Default|GetToMoveGlassUp))
    (Variables|Default|SetSpawnLava true)))

(fn GetRandomPlatformPosition
  (params (Z :type Float%20%28double-precision%29))
  (return (Math|Vector|MakeVector (Math|Random|RandomFloatinRange -1.2e+03 1.2e+03) (Math|Random|RandomFloatinRange -1.2e+03 1.2e+03) Z)))

(fn SpawnEnemiesOverTime
  (params (DT :type Float%20%28double-precision%29) (Z :type Float%20%28double-precision%29))
  ;[0.9623 1 0] Spawns Enemies over time and not all at once
  (if (> (Variables|Default|GetEnemiesDT) 1e+01)
    (bind _returnvalue (Actor|GetActorOfClass "/Game/_TheCubeAssets/Blueprints/Levels/Blank.Blank_C"))
    (for _index (range 0 4)
      (bind _randompos (CallFunction|GetRandomPlatformPosition Z))
      (bind _returnvalue_2 (Game|SpawnActorfromClass "/Game/_TheCubeAssets/Blueprints/Enemies/FlyingRanged_Enemy.FlyingRanged_Enemy_C" (Math|Transform|MakeTransform _randompos) "AdjustIfPossibleButAlwaysSpawn" "MultiplyWithRoot" 0 0))
      (Transformation|AttachActorToActor _returnvalue_2 _returnvalue "None" "KeepRelative" "KeepRelative" "KeepRelative" false))
    (Variables|Default|SetEnemiesDT 0.0)
    (else
      (Variables|Default|SetEnemiesDT (+ (Variables|Default|GetEnemiesDT) DT)))))

(fn GetLevelNumber
  (return (Variables|Default|GetLevel%20Number)))

(fn LevelEnded
  (bind _returnvalue (Actor|GetActorOfClass "/Game/_TheCubeAssets/Blueprints/LevelManager.LevelManager_C"))
  (Default|ClearBlankHolder _returnvalue)
  (if (Variables|Default|GetLevel%20In%20Progress)
    (Development|PrintString (Utilities|String|Append (Utilities|String|Append "Level " (Utilities|String|ToString(Integer) (Variables|Default|GetLevel%20Number))) " ended!"))
    ;[0 1 0.3254] Show Objective
    (bind _asgi_cube_game_instance (Utilities|Casting|CastToGI_CubeGameInstance (Game|GetGameInstance)))
    (bind _aswbp_hud (Utilities|Casting|CastToWBP_HUD (Variables|/Game/_TheCubeAssets/Blueprints/GI_CubeGameInstance.GI_CubeGameInstance_C|GetHUD%20Widget _asgi_cube_game_instance)))
    (Default|CompleteObjective _aswbp_hud (+ (Variables|Default|GetLevel%20Number) 1)))
  (Variables|Default|SetLevel%20In%20Progress false)
  (return))