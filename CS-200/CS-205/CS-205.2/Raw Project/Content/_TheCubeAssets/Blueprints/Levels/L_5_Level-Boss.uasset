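; Boss level actor for level 5, which runs the final boss fight and opens the game-complete map when it is over.
; SpawnLevel teleports the actor into place, then LevelBegin spawns BOSS_Enemy at the world origin and shows the HUD objective through the game instance.
; While the level is in progress, Tick polls the boss reference and loads L_GameComplete once it is invalid.
; LevelEnded completes the objective, but nothing in this graph calls it.
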(event EventBeginPlay
  (Variables|Default|SetLevel%20Number 5))

(event Collision|EventActorBeginOverlap
  (params (OtherActor :type Actor%20Object%20Reference)))

(event EventTick
  (params (DeltaSeconds :type Float%20%28single-precision%29))
  (if (Variables|Default|GetLevel%20In%20Progress)
    (CallFunction|CheckifEnded)))

(event EventLevelBegin
  (CallFunction|SpawnBoss)
  (Variables|Default|SetLevel%20In%20Progress true)
  (Development|PrintString (Utilities|String|Append (Utilities|String|Append "Level " (Utilities|String|ToString(Integer) (Variables|Default|GetLevel%20Number))) " started!"))
  ;[0 1 0.426] Show Objective
  (bind _asgi_cube_game_instance (Utilities|Casting|CastToGI_CubeGameInstance (Game|GetGameInstance)))
  (bind _aswbp_hud (Utilities|Casting|CastToWBP_HUD (Variables|/Game/_TheCubeAssets/Blueprints/GI_CubeGameInstance.GI_CubeGameInstance_C|GetHUD%20Widget _asgi_cube_game_instance)))
  (Default|ShowObjective _aswbp_hud (+ (Variables|Default|GetLevel%20Number) 1)))

(event EventSpawnLevel
  (params (Transform :type Transform))
  (Transformation|SetActorTransform Transform false true)
  (Variables|Default|SetLevel%20In%20Progress false))

(fn ConstructionScript)

(fn SpawnBoss
  (bind _returnvalue (Game|SpawnActorfromClass "/Game/_TheCubeAssets/Blueprints/Enemies/BOSS_Enemy.BOSS_Enemy_C" (Math|Transform|MakeTransform "0, 0, 0") "Undefined" "MultiplyWithRoot" 0 0))
  (Variables|Default|SetBoss _returnvalue))

(fn CheckifEnded
  (if (not (Utilities|IsValid (Variables|Default|GetBoss)))
    (Game|OpenLevel(byObjectReference) "/Game/_TheCubeAssets/Levels/L_GameComplete.L_GameComplete")))

(fn GetLevelNumber
  (return (Variables|Default|GetLevel%20Number)))

(fn LevelEnded
  (if (Variables|Default|GetLevel%20In%20Progress)
    (Development|PrintString (Utilities|String|Append (Utilities|String|Append "Level " (Utilities|String|ToString(Integer) (Variables|Default|GetLevel%20Number))) " ended!"))
    ;[0.731 1 0] Hide Objective
    (bind _asgi_cube_game_instance (Utilities|Casting|CastToGI_CubeGameInstance (Game|GetGameInstance)))
    (bind _aswbp_hud (Utilities|Casting|CastToWBP_HUD (Variables|/Game/_TheCubeAssets/Blueprints/GI_CubeGameInstance.GI_CubeGameInstance_C|GetHUD%20Widget _asgi_cube_game_instance)))
    (Default|CompleteObjective _aswbp_hud (+ (Variables|Default|GetLevel%20Number) 1)))
  (Variables|Default|SetLevel%20In%20Progress false)
  (return))