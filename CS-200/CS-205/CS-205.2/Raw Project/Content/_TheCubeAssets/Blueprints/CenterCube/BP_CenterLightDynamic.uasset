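; Center light effect that spawns a swarm of small cubes, attaches them to itself and keeps them drifting randomly.
; BeginPlay fills parallel arrays of BP_SmallCube actors and target positions.
; Each Tick moves cubes toward their targets with randomized, delta-time-scaled lerps, picking a new target once one is nearly reached.
; Targets are world-space points around the origin, their range modulated by a clamped term from cube scale.
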(event EventBeginPlay
  ;[0.5258 1 0] Spawn Light Cubes
  (Variables|Default|SetCubeMaxRange 5e+01)
  (bind _output_get (Variables|Default|SetNumberOfCubes 50))
  (for _index (range 1 _output_get)
    (bind _returnvalue (Game|SpawnActorfromClass "/Game/_TheCubeAssets/Blueprints/CenterCube/BP_SmallCube.BP_SmallCube_C" (Math|Transform|MakeTransform "0, 0, 0") "Undefined" "MultiplyWithRoot" 0 0))
    (Utilities|Array|Add (Variables|Default|GetLightCubes) _returnvalue)
    ;;[0 0 0] Add blank  target for each cube
    (Utilities|Array|Add :TargetArray (Variables|Default|GetTargetPositions))
    (Transformation|AttachActorToActor _returnvalue self "None" "KeepRelative" "KeepRelative" "KeepRelative" true)))

(event EventTick
  (params (DeltaSeconds :type Float%20%28single-precision%29))
  (bind _cubemaxrange (Variables|Default|GetCubeMaxRange))
  ;[0 0.1893 1] Move the cubes randomly
  (for (_array_element _array_index) (Variables|Default|GetLightCubes)
    (bind _asbp_small_cube (Utilities|Casting|CastToBP_SmallCube _array_element))
    (bind _minimaldifference (CallFunction|CheckifAlmostSame (Transformation|GetActorLocation _array_element) (Utilities|Array|Get(acopy) (Variables|Default|GetTargetPositions) _array_index) 0.5))
    (if _minimaldifference
      (Utilities|Array|SetArrayElem (Variables|Default|GetTargetPositions) _array_index (Math|Vector|MakeVector (Math|Random|RandomFloatinRange (* (* -1.0 _cubemaxrange) (* (Math|Float|Clamp(Float) (- (/ (Variables|Default|GetCubeMaxRange) 2.0) (.X (Math|Vector|BreakVector (Variables|/Script/Engine.SceneComponent|GetRelativeScale3D (Variables|/Game/_TheCubeAssets/Blueprints/CenterCube/BP_SmallCube.BP_SmallCube_C|GetCubeRef _asbp_small_cube)))))) 5.0)) (* _cubemaxrange (* (Math|Float|Clamp(Float) (- (/ (Variables|Default|GetCubeMaxRange) 2.0) (.X (Math|Vector|BreakVector (Variables|/Script/Engine.SceneComponent|GetRelativeScale3D (Variables|/Game/_TheCubeAssets/Blueprints/CenterCube/BP_SmallCube.BP_SmallCube_C|GetCubeRef _asbp_small_cube)))))) 5.0))) (Math|Random|RandomFloatinRange (* (* -1.0 _cubemaxrange) (* (Math|Float|Clamp(Float) (- (/ (Variables|Default|GetCubeMaxRange) 2.0) (.X (Math|Vector|BreakVector (Variables|/Script/Engine.SceneComponent|GetRelativeScale3D (Variables|/Game/_TheCubeAssets/Blueprints/CenterCube/BP_SmallCube.BP_SmallCube_C|GetCubeRef _asbp_small_cube)))))) 5.0)) (* _cubemaxrange (* (Math|Float|Clamp(Float) (- (/ (Variables|Default|GetCubeMaxRange) 2.0) (.X (Math|Vector|BreakVector (Variables|/Script/Engine.SceneComponent|GetRelativeScale3D (Variables|/Game/_TheCubeAssets/Blueprints/CenterCube/BP_SmallCube.BP_SmallCube_C|GetCubeRef _asbp_small_cube)))))) 5.0))) (Math|Random|RandomFloatinRange (* (* -1.0 _cubemaxrange) (* (Math|Float|Clamp(Float) (- (/ (Variables|Default|GetCubeMaxRange) 2.0) (.X (Math|Vector|BreakVector (Variables|/Script/Engine.SceneComponent|GetRelativeScale3D (Variables|/Game/_TheCubeAssets/Blueprints/CenterCube/BP_SmallCube.BP_SmallCube_C|GetCubeRef _asbp_small_cube)))))) 5.0)) (* _cubemaxrange (* (Math|Float|Clamp(Float) (- (/ (Variables|Default|GetCubeMaxRange) 2.0) (.X (Math|Vector|BreakVector (Variables|/Script/Engine.SceneComponent|GetRelativeScale3D (Variables|/Game/_TheCubeAssets/Blueprints/CenterCube/BP_SmallCube.BP_SmallCube_C|GetCubeRef _asbp_small_cube)))))) 5.0)))))
      (else
        (Transformation|SetActorLocation _array_element (Math|Vector|Lerp(Vector) (Transformation|GetActorLocation _array_element) (Utilities|Array|Get(acopy) (Variables|Default|GetTargetPositions) _array_index) (* DeltaSeconds (Math|Random|RandomFloatinRange 0.0 3.0))) false true)))))

(fn ConstructionScript)

(fn CheckifAlmostSame
  (params (R1 :type Vector) (R2 :type Vector) (Tollerance :type Float%20%28double-precision%29))
  (return (Utilities|Operators|EqualEqual R1 R2 Tollerance)))