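; MovingCube_BP is a cube hazard that roams along the X and Y axes and damages the first-person character on overlap while its material is Lava.
; MoveCube picks a random direction, plays that axis timeline as an offset from the start location, then calls itself on finish.
; A projectile hit turns the cube to steel and stops it.
; Other overlaps reverse it, and overlapped cubes are set to Lava.
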(event OnComponentEndOverlap(Box)
  (params (OverlappedComponent :type Primitive%20Component%20Object%20Reference) (OtherActor :type Actor%20Object%20Reference) (OtherComp :type Primitive%20Component%20Object%20Reference) (OtherBodyIndex :type Integer))
  ;[1 1 1] Resets Material when Cubes No longer collide
  (bind _asmoving_cube_bp (Utilities|Casting|CastToMovingCube_BP OtherActor))
  (Rendering|Material|SetMaterial (Variables|MovingCube_BP_C|GetCube _asmoving_cube_bp) 0 "/Game/_TheCubeAssets/Materials/Platformer_Level/Lava.Lava"))

(event OnComponentBeginOverlap(Box)
  (params (OverlappedComponent :type Primitive%20Component%20Object%20Reference) (OtherActor :type Actor%20Object%20Reference) (OtherComp :type Primitive%20Component%20Object%20Reference) (OtherBodyIndex :type Integer) (bFromSweep :type Boolean) (SweepResult :type Hit%20Result%20Structure%20%28by%20ref%29))
  ;[1 1 1] When bullet hits cube get current direction and stop timeline or if not bullet reverse timeline
  (bind _asbp_first_person_character (Utilities|Casting|CastToBP_FirstPersonCharacter OtherActor)
    (:then
      (bind _asmoving_cube_bp (Utilities|Casting|CastToMovingCube_BP self))
      (if (== (Rendering|Material|GetMaterial (Variables|MovingCube_BP_C|GetCube _asmoving_cube_bp) 0) "/Game/_TheCubeAssets/Materials/Platformer_Level/Lava.Lava")
        (Default|TakeDamage _asbp_first_person_character 5.0)))
    (:CastFailed
      (Utilities|Casting|CastToBP_FirstPersonProjectile OtherActor
        (:then
          (Rendering|Material|SetMaterial (Variables|Default|GetCube) 0 "/Game/StarterContent/Materials/M_Metal_Burnished_Steel.M_Metal_Burnished_Steel")
          (switch int (Variables|Default|GetDirectionChoice)
            (:0
              ;[1 1 1] Timeline is same just changes the Direction of Cube movement each time
              (bind _x_axis (Timeline|Timeline_0 Stop)
                (:Update
                  (Transformation|SetActorLocation (+ (Variables|Default|GetStartLocation) (Math|Vector|MakeVector _x_axis 0.0 0.0)) false false))
                (:Finished
                  (CallFunction|MoveCube))))
            (:1
              (bind _axis (Timeline|Timeline_1 Stop)
                (:Update
                  (Transformation|SetActorLocation (+ (Variables|Default|GetStartLocation) (Math|Vector|MakeVector 0.0 _axis 0.0)) false false))
                (:Finished
                  (CallFunction|MoveCube))))
            (:2
              (bind _x_axis_2 (Timeline|Timeline_2 Stop)
                (:Update
                  (Transformation|SetActorLocation (+ (Variables|Default|GetStartLocation) (Math|Vector|MakeVector 0.0 (* _x_axis_2 -1.0) 0.0)) false false))
                (:Finished
                  (CallFunction|MoveCube))))
            (:3
              (bind _x_axis_3 (Timeline|Timeline_3 Stop)
                (:Update
                  (Transformation|SetActorLocation (+ (Variables|Default|GetStartLocation) (Math|Vector|MakeVector (* _x_axis_3 -1.0) 0.0 0.0)) false false))
                (:Finished
                  (CallFunction|MoveCube))))))
        (:CastFailed
          (bind _asmoving_cube_bp_2 (Utilities|Casting|CastToMovingCube_BP OtherActor)
            (:then
              (Rendering|Material|SetMaterial (Variables|MovingCube_BP_C|GetCube _asmoving_cube_bp_2) 0 "/Game/_TheCubeAssets/Materials/Platformer_Level/Lava.Lava"))
            (:CastFailed
              _))
          (switch int (Variables|Default|GetDirectionChoice)
            (:0
              (Timeline|Timeline_0 Reverse))
            (:1
              (Timeline|Timeline_1 Reverse))
            (:2
              (Timeline|Timeline_2 Reverse))
            (:3
              (Timeline|Timeline_3 Reverse))))))))

(event Custom|MoveCube
  ;[1 1 1] Set Play Rate(Multiplied) of timelines and randomly select Direction, Set hit to False
  (Variables|Default|SetStartLocation (Transformation|GetActorLocation))
  (Components|Timeline|SetPlayRate (Variables|Default|GetTimeline_3) 5.0)
  (bind _output_get (Variables|Default|SetDirectionChoice (Math|Random|RandomIntegerinRange 0 3)))
  (switch int _output_get
    (:0
      ;[1 1 1] Timeline is same just changes the Direction of Cube movement each time
      (bind _x_axis (Timeline|Timeline_0 PlayFromStart)
        (:Update
          (Transformation|SetActorLocation (+ (Variables|Default|GetStartLocation) (Math|Vector|MakeVector _x_axis 0.0 0.0)) false false))
        (:Finished
          (CallFunction|MoveCube))))
    (:1
      (bind _axis (Timeline|Timeline_1 PlayFromStart)
        (:Update
          (Transformation|SetActorLocation (+ (Variables|Default|GetStartLocation) (Math|Vector|MakeVector 0.0 _axis 0.0)) false false))
        (:Finished
          (CallFunction|MoveCube))))
    (:2
      (bind _x_axis_2 (Timeline|Timeline_2 PlayFromStart)
        (:Update
          (Transformation|SetActorLocation (+ (Variables|Default|GetStartLocation) (Math|Vector|MakeVector 0.0 (* _x_axis_2 -1.0) 0.0)) false false))
        (:Finished
          (CallFunction|MoveCube))))
    (:3
      (bind _x_axis_3 (Timeline|Timeline_3 PlayFromStart)
        (:Update
          (Transformation|SetActorLocation (+ (Variables|Default|GetStartLocation) (Math|Vector|MakeVector (* _x_axis_3 -1.0) 0.0 0.0)) false false))
        (:Finished
          (CallFunction|MoveCube))))))

(fn ConstructionScript)