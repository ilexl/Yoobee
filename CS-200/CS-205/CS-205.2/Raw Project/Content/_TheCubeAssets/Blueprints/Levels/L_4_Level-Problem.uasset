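; Level 4 actor for a key-hunt stage: collecting ten keys tells LevelManager to advance.
; LevelBegin shows the HUD objective, builds a tile grid over spawned lava and starts a looping ten-second timer.
; Each cycle destroys previous items, randomly makes about one in five tiles pulse, and spawns pickups on those tiles.
; Pulse material marks spawn tiles; the random range yields keys, health or weapon-1 ammo, leaving the weapon-2 case unreachable.
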(event EventBeginPlay
  (Variables|Default|SetLevel%20Number 4))

(event Collision|EventActorBeginOverlap
  (params (OtherActor :type Actor%20Object%20Reference)))

(event EventTick
  (params (DeltaSeconds :type Float%20%28single-precision%29))
  (if (Variables|Default|GetLevel%20In%20Progress)
    (CallFunction|CheckKeys)))

(event EventLevelBegin
  (Variables|Default|SetLevel%20In%20Progress true)
  (Development|PrintString (Utilities|String|Append (Utilities|String|Append "Level " (Utilities|String|ToString(Integer) (Variables|Default|GetLevel%20Number))) " started!"))
  ;[0 1 0.2201] Show Objective
  (bind _asgi_cube_game_instance (Utilities|Casting|CastToGI_CubeGameInstance (Game|GetGameInstance)))
  (bind _aswbp_hud (Utilities|Casting|CastToWBP_HUD (Variables|/Game/_TheCubeAssets/Blueprints/GI_CubeGameInstance.GI_CubeGameInstance_C|GetHUD%20Widget _asgi_cube_game_instance)))
  (Default|ShowObjective _aswbp_hud (+ (Variables|Default|GetLevel%20Number) 1))
  ;[1 1 1] Calls relevant functions and Spawns Lava on floor
  (CallFunction|GridGenerator)
  (CallFunction|Timer)
  (bind _returnvalue (Actor|GetActorOfClass "/Game/_TheCubeAssets/Blueprints/Levels/Blank.Blank_C"))
  (bind _returnvalue_2 (Game|SpawnActorfromClass "/Game/_TheCubeAssets/Blueprints/Levels/L_4-Problem/Lava_BP.Lava_BP_C" (Math|Transform|MakeTransform (Math|Vector|MakeVector 0.0 0.0 -1.99e+03)) "Undefined" "MultiplyWithRoot" 0 0))
  (Transformation|AttachActorToActor _returnvalue_2 _returnvalue "None" "KeepRelative" "KeepRelative" "KeepRelative" true)
  (Utilities|Array|Clear (Variables|Default|GetItems))
  (CallFunction|Repeat))

(event EventSpawnLevel
  (params (Transform :type Transform))
  (Transformation|SetActorTransform Transform false true)
  (Variables|Default|SetLevel%20In%20Progress false))

(fn ConstructionScript)

(fn GridGenerator
  (bind _grid_size (Variables|Default|GetGrid%20Size))
  (bind _grid_size_2 (Variables|Default|GetGrid%20Size))
  (bind _returnvalue (/ _grid_size_2 2))
  (bind _returnvalue_2 (* _returnvalue 420))
  (bind _returnvalue_3 (- 0 _returnvalue_2))
  (bind _returnvalue_4 (Math|Conversions|ToFloat(Integer) _returnvalue_3))
  (Variables|Default|SetX _returnvalue_4)
  (Variables|Default|SetY _returnvalue_4)
  (bind _output_get (Variables|Default|SetStart_X _returnvalue_4))
  (for _index (range 0 _grid_size)
    (for _index_2 (range 0 _grid_size)
      (Game|SpawnActorfromClass "/Game/_TheCubeAssets/Blueprints/Levels/L_4-Problem/GridTiles_BP.GridTiles_BP_C" (Math|Transform|MakeTransform (Math|Vector|MakeVector (Variables|Default|GetX) (Variables|Default|GetY) -1.95e+03)) "Undefined" "MultiplyWithRoot" 0 0)
      (Variables|Default|SetX (+ (Variables|Default|GetX) 4.2e+02)))
    (Variables|Default|SetX _output_get)
    (Variables|Default|SetY (+ (Variables|Default|GetY) 4.2e+02)))
  (bind _outactors (Actor|GetAllActorsOfClass "/Game/_TheCubeAssets/Blueprints/Levels/L_4-Problem/GridTiles_BP.GridTiles_BP_C"))
  (for _array_element _outactors
    (bind _returnvalue_5 (Actor|GetActorOfClass "/Game/_TheCubeAssets/Blueprints/Levels/Blank.Blank_C"))
    (Transformation|AttachActorToActor _array_element _returnvalue_5 "None" "KeepRelative" "KeepRelative" "KeepRelative" false)))

(fn GridMatColour
  ;[1 1 1] Gets All Grid Tiles and assigns colour between Brown or Red (Mainly Brown)
  (bind _outactors (Actor|GetAllActorsOfClass "/Game/_TheCubeAssets/Blueprints/Levels/L_4-Problem/GridTiles_BP.GridTiles_BP_C"))
  (for _array_element _outactors
    (switch int (Math|Random|RandomInteger 5)
      (:0
        (Rendering|Material|SetMaterial (Variables|/Game/_TheCubeAssets/Blueprints/Levels/L_4-Problem/GridTiles_BP.GridTiles_BP_C|GetCube _array_element) 0 "/Game/StarterContent/Materials/M_Tech_Hex_Tile.M_Tech_Hex_Tile"))
      (:1
        (Rendering|Material|SetMaterial (Variables|/Game/_TheCubeAssets/Blueprints/Levels/L_4-Problem/GridTiles_BP.GridTiles_BP_C|GetCube _array_element) 0 "/Game/StarterContent/Materials/M_Tech_Hex_Tile.M_Tech_Hex_Tile"))
      (:2
        (Rendering|Material|SetMaterial (Variables|/Game/_TheCubeAssets/Blueprints/Levels/L_4-Problem/GridTiles_BP.GridTiles_BP_C|GetCube _array_element) 0 "/Game/StarterContent/Materials/M_Tech_Hex_Tile.M_Tech_Hex_Tile"))
      (:3
        (Rendering|Material|SetMaterial (Variables|/Game/_TheCubeAssets/Blueprints/Levels/L_4-Problem/GridTiles_BP.GridTiles_BP_C|GetCube _array_element) 0 "/Game/StarterContent/Materials/M_Tech_Hex_Tile.M_Tech_Hex_Tile"))
      (:4
        (Rendering|Material|SetMaterial (Variables|/Game/_TheCubeAssets/Blueprints/Levels/L_4-Problem/GridTiles_BP.GridTiles_BP_C|GetCube _array_element) 0 "/Game/StarterContent/Materials/M_Tech_Hex_Tile_Pulse.M_Tech_Hex_Tile_Pulse")))))

(fn Timer
  ;[1 1 1] Sets Timer Every 10 seconds Changes those colours by calling function
  (Utilities|Time|SetTimerbyFunctionName 0 "Repeat" 1e+01 true))

(fn ItemSpawner
  (params (ArrayOfTiles :type Array%20of%20Grid%20Tiles%20BP%20Object%20References))
  (bind _returnvalue (Actor|GetActorOfClass "/Game/_TheCubeAssets/Blueprints/Levels/Blank.Blank_C"))
  (for _array_element ArrayOfTiles
    ;[1 1 1] Randomly Selects and item to spawn, Spawn at Hex Coloured Grid Tile, Adds item to array
    (if (== (Rendering|Material|GetMaterial (Actor|GetComponentbyClass _array_element "/Script/Engine.StaticMeshComponent") 0) "/Game/StarterContent/Materials/M_Tech_Hex_Tile_Pulse.M_Tech_Hex_Tile_Pulse")
      (switch int (Math|Random|RandomInteger 3)
        (:0
          (bind _returnvalue_2 (Game|SpawnActorfromClass "/Game/_TheCubeAssets/Blueprints/Items/BP_Key.BP_Key_C" (Math|Conversions|ToTransform(Vector) (Math|Transform|TransformLocation (Math|Conversions|ToTransform(Vector) (Transformation|GetActorLocation _array_element)) "0.000000,0.000000,50.000000")) "AdjustIfPossibleButAlwaysSpawn" "MultiplyWithRoot" 0 0))
          (Transformation|AttachActorToActor _returnvalue_2 _returnvalue "None" "KeepRelative" "KeepRelative" "KeepRelative" true)
          (Utilities|Array|Add (Variables|Default|GetItems) _returnvalue_2))
        (:1
          (bind _returnvalue_3 (Game|SpawnActorfromClass "/Game/_TheCubeAssets/Blueprints/Items/BP_Health.BP_Health_C" (Math|Conversions|ToTransform(Vector) (Math|Transform|TransformLocation (Math|Conversions|ToTransform(Vector) (Transformation|GetActorLocation _array_element)) "0.000000,0.000000,50.000000")) "AdjustIfPossibleButAlwaysSpawn" "MultiplyWithRoot" 0 0))
          (Transformation|AttachActorToActor _returnvalue_3 _returnvalue "None" "KeepRelative" "KeepRelative" "KeepRelative" true)
          (Utilities|Array|Add (Variables|Default|GetItems) _returnvalue_3))
        (:2
          (bind _returnvalue_4 (Game|SpawnActorfromClass "/Game/_TheCubeAssets/Blueprints/Items/BP_Ammo_Weapon1.BP_Ammo_Weapon1_C" (Math|Conversions|ToTransform(Vector) (Math|Transform|TransformLocation (Math|Conversions|ToTransform(Vector) (Transformation|GetActorLocation _array_element)) "0.000000,0.000000,50.000000")) "Undefined" "MultiplyWithRoot" 0 0))
          (Transformation|AttachActorToActor _returnvalue_4 _returnvalue "None" "KeepRelative" "KeepRelative" "KeepRelative" true)
          (Utilities|Array|Add (Variables|Default|GetItems) _returnvalue_4))
        (:3
          (bind _returnvalue_5 (Game|SpawnActorfromClass "/Game/_TheCubeAssets/Blueprints/Items/BP_Ammo_Weapon2.BP_Ammo_Weapon2_C" (Math|Conversions|ToTransform(Vector) (Math|Transform|TransformLocation (Math|Conversions|ToTransform(Vector) (Transformation|GetActorLocation _array_element)) "0.000000,0.000000,50.000000")) "Undefined" "MultiplyWithRoot" 0 0))
          (Transformation|AttachActorToActor _returnvalue_5 _returnvalue "None" "KeepRelative" "KeepRelative" "KeepRelative" true)
          (Utilities|Array|Add (Variables|Default|GetItems) _returnvalue_5))))))

(fn DeleteItems
  (for _array_element (Variables|Default|GetItems)
    (if (Utilities|IsValid _array_element)
      (Actor|DestroyActor _array_element))))

(fn Repeat
  (CallFunction|DeleteItems)
  (CallFunction|GridMatColour)
  (bind _outactors (Actor|GetAllActorsOfClass "/Game/_TheCubeAssets/Blueprints/Levels/L_4-Problem/GridTiles_BP.GridTiles_BP_C"))
  (CallFunction|ItemSpawner _outactors))

(fn CheckKeys
  (if (== (Variables|Default|GetAmountCollectedKeys) 10)
    (bind _returnvalue (Actor|GetActorOfClass "/Game/_TheCubeAssets/Blueprints/LevelManager.LevelManager_C"))
    (Default|NextLevel _returnvalue)))

(fn CollectedKeys
  (Math|Integer|IncrementInt (Variables|Default|GetAmountCollectedKeys)
    (:%20%20
      (CallFunction|CheckKeys))))

(fn GetLevelNumber
  (return (Variables|Default|GetLevel%20Number)))

(fn LevelEnded
  (if (Variables|Default|GetLevel%20In%20Progress)
    (Development|PrintString (Utilities|String|Append (Utilities|String|Append "Level " (Utilities|String|ToString(Integer) (Variables|Default|GetLevel%20Number))) " ended!"))
    ;[1 0.925 0] Complete Objective
    (bind _asgi_cube_game_instance (Utilities|Casting|CastToGI_CubeGameInstance (Game|GetGameInstance)))
    (bind _aswbp_hud (Utilities|Casting|CastToWBP_HUD (Variables|/Game/_TheCubeAssets/Blueprints/GI_CubeGameInstance.GI_CubeGameInstance_C|GetHUD%20Widget _asgi_cube_game_instance)))
    (Default|CompleteObjective _aswbp_hud (+ (Variables|Default|GetLevel%20Number) 1)))
  (Variables|Default|SetLevel%20In%20Progress false)
  (return))