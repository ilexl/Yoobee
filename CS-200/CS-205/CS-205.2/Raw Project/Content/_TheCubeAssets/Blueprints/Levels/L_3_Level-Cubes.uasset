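; Level 3 controller actor for the cube game, a stage of moving cubes where every key must be collected.
; LevelBegin shows the HUD objective, builds a centred tile grid and cube grid, starts the cubes moving, then places four platforms and four keys, attaching everything to the Blank actor.
; While the level runs, Tick polls for remaining keys and calls LevelManager's NextLevel when none are left.
; LevelEnded completes the HUD objective and clears the in-progress flag.
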(event EventBeginPlay
  (Variables|Default|SetLevel%20Number 3))

(event Collision|EventActorBeginOverlap
  (params (OtherActor :type Actor%20Object%20Reference)))

(event EventTick
  (params (DeltaSeconds :type Float%20%28single-precision%29))
  (if (Variables|Default|GetLevel%20In%20Progress)
    (CallFunction|CheckKeys)))

(event EventLevelBegin
  (Variables|Default|SetLevel%20In%20Progress true)
  (Development|PrintString (Utilities|String|Append (Utilities|String|Append "Level " (Utilities|String|ToString(Integer) (Variables|Default|GetLevel%20Number))) " started!"))
  ;[0 1 0.009441] Show Objective
  (bind _asgi_cube_game_instance (Utilities|Casting|CastToGI_CubeGameInstance (Game|GetGameInstance)))
  (bind _aswbp_hud (Utilities|Casting|CastToWBP_HUD (Variables|/Game/_TheCubeAssets/Blueprints/GI_CubeGameInstance.GI_CubeGameInstance_C|GetHUD%20Widget _asgi_cube_game_instance)))
  (Default|ShowObjective _aswbp_hud (+ (Variables|Default|GetLevel%20Number) 1))
  ;[0.3898 1 0] Create level assets
  (CallFunction|GridGenerator)
  (CallFunction|SpawnCube)
  (bind _outactors (Actor|GetAllActorsOfClass "/Game/_TheCubeAssets/Blueprints/Levels/L_3-Cubes/MovingCube_BP.MovingCube_BP_C"))
  (for _array_element _outactors
    (Default|MoveCube _array_element))
  (CallFunction|SpawnPlatform)
  (CallFunction|ItemSpawn))

(event EventSpawnLevel
  (params (Transform :type Transform))
  (Transformation|SetActorTransform Transform false true)
  (Variables|Default|SetLevel%20In%20Progress false))

(fn ConstructionScript)

(fn GridGenerator
  (bind _grid_size (Variables|Default|GetGrid%20Size))
  (bind _grid_size_2 (Variables|Default|GetGrid%20Size))
  (bind _returnvalue (/ _grid_size_2 2))
  (bind _returnvalue_2 (* _returnvalue 880))
  (bind _returnvalue_3 (- 0 _returnvalue_2))
  (bind _returnvalue_4 (Math|Conversions|ToFloat(Integer) _returnvalue_3))
  ;[0.06641 1 0.6819] Grid Code
  (Variables|Default|SetX _returnvalue_4)
  (Variables|Default|SetY _returnvalue_4)
  (bind _output_get (Variables|Default|SetX_Start _returnvalue_4))
  (for _index (range 0 _grid_size)
    (for _index_2 (range 0 _grid_size)
      (Game|SpawnActorfromClass "/Game/_TheCubeAssets/Blueprints/Levels/L_3-Cubes/GridTile_BP.GridTile_BP_C" (Math|Transform|MakeTransform (Math|Vector|MakeVector (Variables|Default|GetX) (Variables|Default|GetY) -1.99e+03)) "Undefined" "MultiplyWithRoot" 0 0)
      (Variables|Default|SetX (+ (Variables|Default|GetX) 8.8e+02)))
    (Variables|Default|SetX _output_get)
    (Variables|Default|SetY (+ (Variables|Default|GetY) 8.8e+02)))
  (bind _outactors (Actor|GetAllActorsOfClass "/Game/_TheCubeAssets/Blueprints/Levels/L_3-Cubes/GridTile_BP.GridTile_BP_C"))
  (for _array_element _outactors
    (bind _returnvalue_5 (Actor|GetActorOfClass "/Game/_TheCubeAssets/Blueprints/Levels/Blank.Blank_C"))
    (Transformation|AttachActorToActor _array_element _returnvalue_5 "None" "KeepRelative" "KeepRelative" "KeepRelative" false)))

(fn SpawnCube
  (bind _amount_cubes (Variables|Default|GetAmount%20Cubes))
  (bind _amount_cubes_2 (Variables|Default|GetAmount%20Cubes))
  (bind _returnvalue (/ _amount_cubes 2))
  (bind _returnvalue_2 (* _returnvalue 880))
  (bind _returnvalue_3 (- 0 _returnvalue_2))
  (bind _returnvalue_4 (Math|Conversions|ToFloat(Integer) _returnvalue_3))
  ;[1 0.7945 0] Spawns Moving Cubes
  (Variables|Default|SetX _returnvalue_4)
  (Variables|Default|SetY _returnvalue_4)
  (bind _output_get (Variables|Default|SetX_Start _returnvalue_4))
  (for _index (range 0 _amount_cubes_2)
    (for _index_2 (range 0 _amount_cubes_2)
      (bind _returnvalue_5 (Game|SpawnActorfromClass "/Game/_TheCubeAssets/Blueprints/Levels/L_3-Cubes/MovingCube_BP.MovingCube_BP_C" (Math|Transform|MakeTransform (Math|Vector|MakeVector (Variables|Default|GetX) (Variables|Default|GetY) -1.99e+03)) "Undefined" "MultiplyWithRoot" 0 0))
      (Variables|Default|SetX (+ (Variables|Default|GetX) 8.8e+02))
      (bind _returnvalue_6 (Actor|GetActorOfClass "/Game/_TheCubeAssets/Blueprints/Levels/Blank.Blank_C"))
      (Transformation|AttachActorToActor _returnvalue_5 _returnvalue_6 "None" "KeepRelative" "KeepRelative" "KeepRelative" false))
    (Variables|Default|SetX _output_get)
    (Variables|Default|SetY (+ (Variables|Default|GetY) 8.8e+02))))

(fn SpawnPlatform
  ;[0 1 0.004232] Spawns Platforms
  (bind _returnvalue (Game|SpawnActorfromClass "/Game/_TheCubeAssets/Blueprints/Levels/L_3-Cubes/Platform_BP.Platform_BP_C" (Math|Transform|MakeTransform (Math|Vector|MakeVector 4e+02 -1.8e+03 -1.65e+03)) "Undefined" "MultiplyWithRoot" 0 0))
  (bind _returnvalue_2 (Game|SpawnActorfromClass "/Game/_TheCubeAssets/Blueprints/Levels/L_3-Cubes/Platform_BP.Platform_BP_C" (Math|Transform|MakeTransform (Math|Vector|MakeVector 4e+02 1.8e+03 -1.65e+03)) "Undefined" "MultiplyWithRoot" 0 0))
  (bind _returnvalue_3 (Game|SpawnActorfromClass "/Game/_TheCubeAssets/Blueprints/Levels/L_3-Cubes/Platform_BP.Platform_BP_C" (Math|Transform|MakeTransform (Math|Vector|MakeVector 1.8e+03 4e+02 -1.65e+03) "0.000000,90.000000,0.000000") "Undefined" "MultiplyWithRoot" 0 0))
  (bind _returnvalue_4 (Game|SpawnActorfromClass "/Game/_TheCubeAssets/Blueprints/Levels/L_3-Cubes/Platform_BP.Platform_BP_C" (Math|Transform|MakeTransform (Math|Vector|MakeVector -1.8e+03 -4e+02 -1.65e+03) "0.000000,-90.000000,0.000000") "Undefined" "MultiplyWithRoot" 0 0))
  (bind _returnvalue_5 (Actor|GetActorOfClass "/Game/_TheCubeAssets/Blueprints/Levels/Blank.Blank_C"))
  (Transformation|AttachActorToActor _returnvalue_3 _returnvalue_5 "None" "KeepRelative" "KeepRelative" "KeepRelative" false)
  (Transformation|AttachActorToActor _returnvalue_2 _returnvalue_5 "None" "KeepRelative" "KeepRelative" "KeepRelative" false)
  (Transformation|AttachActorToActor _returnvalue_4 _returnvalue_5 "None" "KeepRelative" "KeepRelative" "KeepRelative" false)
  (Transformation|AttachActorToActor _returnvalue _returnvalue_5 "None" "KeepRelative" "KeepRelative" "KeepRelative" false))

(fn ItemSpawn
  ;[0.5716 1 0] Spawns Items
  (bind _returnvalue (Game|SpawnActorfromClass "/Game/_TheCubeAssets/Blueprints/Items/BP_Key.BP_Key_C" (Math|Transform|MakeTransform (Math|Vector|MakeVector 0.0 -1.8e+03 -1.6e+03)) "AdjustIfPossibleButAlwaysSpawn" "MultiplyWithRoot" 0 0))
  (bind _returnvalue_2 (Game|SpawnActorfromClass "/Game/_TheCubeAssets/Blueprints/Items/BP_Key.BP_Key_C" (Math|Transform|MakeTransform (Math|Vector|MakeVector 0.0 1.8e+03 -1.6e+03)) "AdjustIfPossibleButAlwaysSpawn" "MultiplyWithRoot" 0 0))
  (bind _returnvalue_3 (Game|SpawnActorfromClass "/Game/_TheCubeAssets/Blueprints/Items/BP_Key.BP_Key_C" (Math|Transform|MakeTransform (Math|Vector|MakeVector 1.8e+03 0.0 -1.6e+03) "0.000000,90.000000,0.000000") "AdjustIfPossibleButAlwaysSpawn" "MultiplyWithRoot" 0 0))
  (bind _returnvalue_4 (Game|SpawnActorfromClass "/Game/_TheCubeAssets/Blueprints/Items/BP_Key.BP_Key_C" (Math|Transform|MakeTransform (Math|Vector|MakeVector -1.8e+03 0.0 -1.6e+03) "0.000000,-90.000000,0.000000") "AdjustIfPossibleButAlwaysSpawn" "MultiplyWithRoot" 0 0))
  (bind _returnvalue_5 (Actor|GetActorOfClass "/Game/_TheCubeAssets/Blueprints/Levels/Blank.Blank_C"))
  (Transformation|AttachActorToActor _returnvalue_4 _returnvalue_5 "None" "KeepRelative" "KeepRelative" "KeepRelative" false)
  (Transformation|AttachActorToActor _returnvalue_3 _returnvalue_5 "None" "KeepRelative" "KeepRelative" "KeepRelative" false)
  (Transformation|AttachActorToActor _returnvalue_2 _returnvalue_5 "None" "KeepRelative" "KeepRelative" "KeepRelative" false)
  (Transformation|AttachActorToActor _returnvalue _returnvalue_5 "None" "KeepRelative" "KeepRelative" "KeepRelative" false))

(fn CheckKeys
  (bind _outactors (Actor|GetAllActorsOfClass "/Game/_TheCubeAssets/Blueprints/Items/BP_Key.BP_Key_C"))
  (if (== (Utilities|Array|Length _outactors) 0)
    (bind _returnvalue (Actor|GetActorOfClass "/Game/_TheCubeAssets/Blueprints/LevelManager.LevelManager_C"))
    (Default|NextLevel _returnvalue)))

(fn GetLevelNumber
  (return (Variables|Default|GetLevel%20Number)))

(fn LevelEnded
  (if (Variables|Default|GetLevel%20In%20Progress)
    (Development|PrintString (Utilities|String|Append (Utilities|String|Append "Level " (Utilities|String|ToString(Integer) (Variables|Default|GetLevel%20Number))) " ended!"))
    ;[1 0.977 0] Complete Objective
    (bind _asgi_cube_game_instance (Utilities|Casting|CastToGI_CubeGameInstance (Game|GetGameInstance)))
    (bind _aswbp_hud (Utilities|Casting|CastToWBP_HUD (Variables|/Game/_TheCubeAssets/Blueprints/GI_CubeGameInstance.GI_CubeGameInstance_C|GetHUD%20Widget _asgi_cube_game_instance)))
    (Default|CompleteObjective _aswbp_hud (+ (Variables|Default|GetLevel%20Number) 1)))
  (Variables|Default|SetLevel%20In%20Progress false)
  (return))