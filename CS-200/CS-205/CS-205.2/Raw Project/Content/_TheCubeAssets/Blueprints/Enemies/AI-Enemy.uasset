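; AI controller for enemies that starts their behavior tree when it possesses a pawn.
; After a short delay it casts the pawn to the ranged, flying ranged or boss enemy class; all three run the same ranged behavior tree.
; It then stores the player character in the Blackboard's Player key, or prints a warning for any other pawn class.
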(event EventPossess
  (params (PossessedPawn :type Pawn%20Object%20Reference))
  ;[1 0.8702 0] Behaviour for Enemies
  (Utilities|FlowControl|Delay 0.1)
  (Utilities|Casting|CastToRanged_Enemy PossessedPawn
    (:then
      (AI|RunBehaviorTree "/Game/_TheCubeAssets/Blueprints/Enemies/BT_Enemy_Ranged.BT_Enemy_Ranged")
      (AI|Components|Blackboard|SetValueasObject (Variables|Default|GetBlackboard) (Utilities|Name|MakeLiteralName "Player") (Game|GetPlayerCharacter 0) :!label _label))
    (:CastFailed
      (Utilities|Casting|CastToFlyingRanged_Enemy PossessedPawn
        (:then
          (AI|RunBehaviorTree "/Game/_TheCubeAssets/Blueprints/Enemies/BT_Enemy_Ranged.BT_Enemy_Ranged")
          (goto _label))
        (:CastFailed
          (Utilities|Casting|CastToBOSS_Enemy PossessedPawn
            (:then
              (AI|RunBehaviorTree "/Game/_TheCubeAssets/Blueprints/Enemies/BT_Enemy_Ranged.BT_Enemy_Ranged")
              (goto _label))
            (:CastFailed
              (Development|PrintText "No Enemy Class Selected in AI-Enemy"))))))))

(fn ConstructionScript)