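; Wave-survival level actor for level 1, which shows and completes its HUD objective as it begins and ends.
; While in progress, Tick lerps spawned barriers upward, then spawns ranged enemies in timed batches at random points scaled to the mesh, slowing after the first batches.
; Once spawning finishes and no ranged or flying enemies remain, it calls NextLevel on LevelManager.
; Spawns attach to a Blank holder actor, which LevelEnded clears through LevelManager.
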(event EventBeginPlay
  (Variables|Components|SetLevel%20Number 1))

(event Collision|EventActorBeginOverlap
  (params (OtherActor :type Actor%20Object%20Reference)))

(event EventTick
  (params (DeltaSeconds :type Float%20%28single-precision%29))
  ;[1 0.8376 0] Level Loop
  (if (Variables|Default|GetLevel%20In%20Progress)
    (CallFunction|RaiseBarriers DeltaSeconds)
    (CallFunction|SpawnEnemiesOverTime DeltaSeconds)
    (CallFunction|CheckifLevelEnded)))

(event EventLevelBegin
  (Variables|Default|SetLevel%20In%20Progress true)
  (Development|PrintString (Utilities|String|Append (Utilities|String|Append "Level " (Utilities|String|ToString(Integer) (Variables|Components|GetLevel%20Number))) " started!"))
  ;[0 1 0.4551] Show Objective
  (bind _asgi_cube_game_instance (Utilities|Casting|CastToGI_CubeGameInstance (Game|GetGameInstance)))
  (bind _aswbp_hud (Utilities|Casting|CastToWBP_HUD (Variables|/Game/_TheCubeAssets/Blueprints/GI_CubeGameInstance.GI_CubeGameInstance_C|GetHUD%20Widget _asgi_cube_game_instance)))
  (Default|ShowObjective _aswbp_hud (+ (Variables|Components|GetLevel%20Number) 1))
  ;[0.4349 0 1] Start of Level
  (Variables|Default|SetRaise true)
  (Variables|Default|SetRaiseComplete false)
  (Variables|Default|SetSpawning%20Complete false))

(event EventSpawnLevel
  (params (Transform :type Transform))
  (Transformation|SetActorTransform Transform false true)
  (Variables|Default|SetLevel%20In%20Progress false))

(fn ConstructionScript)

(fn RandomLocation
  (bind _returnvalue (Transformation|GetActorTransform))
  (bind _staticmesh (Variables|Default|GetStaticMesh))
  (bind _location (Math|Transform|BreakTransform _returnvalue))
  (bind _returnvalue_2 (Transformation|GetRelativeTransform _staticmesh))
  (bind _scale (Math|Transform|BreakTransform _returnvalue_2))
  (bind _z (Math|Vector|BreakVector _location))
  (bind (_x _y) (Math|Vector|BreakVector _scale))
  (bind _returnvalue_3 (+ _z 1e+02))
  (bind _returnvalue_4 (* _y 5e+01))
  (bind _returnvalue_5 (* _x 5e+01))
  (bind _returnvalue_6 (- _returnvalue_4 5e+01))
  (bind _returnvalue_7 (- _returnvalue_5 5e+01))
  (bind _returnvalue_8 (* _returnvalue_6 -1.0))
  (bind _returnvalue_9 (* _returnvalue_7 -1.0))
  (bind _returnvalue_10 (Math|Random|RandomFloatinRange _returnvalue_8 _returnvalue_6))
  (bind _returnvalue_11 (Math|Random|RandomFloatinRange _returnvalue_9 _returnvalue_7))
  (bind _returnvalue_12 (Math|Vector|MakeVector _returnvalue_11 _returnvalue_10 _returnvalue_3))
  ;[1 0.2216 0] Returns a random location
  (Development|PrintString (Utilities|String|ToString(Vector) _returnvalue_12))
  (return (Math|Transform|MakeTransform _returnvalue_12)))

(fn RaiseBarriers
  (params (DT :type Float%20%28double-precision%29))
  ;[1 0.7392 0] Raises Barriers for player defense
  (if (Variables|Default|GetRaise)
    (if (Variables|Default|GetRaiseComplete)
      (return)
      (else
        (bind _returnvalue (Actor|GetActorOfClass "/Game/_TheCubeAssets/Blueprints/Levels/L_1-Waves/Waves-Barriers.Waves-Barriers_C"))
        (if (Utilities|IsValid _returnvalue)
          (Transformation|SetActorLocation _returnvalue (Math|Vector|Lerp(Vector) (Transformation|GetActorLocation _returnvalue) "0.000000,0.000000,-1950.000000" DT) false true)
          (if (< (Math|Vector|Distance(Vector) "0.000000,0.000000,-1950.000000" (Math|Vector|Lerp(Vector) (Transformation|GetActorLocation _returnvalue) "0.000000,0.000000,-1950.000000" DT)) 5.0)
            (Variables|Default|SetRaiseComplete true))
          (else
            (bind _returnvalue_2 (Game|SpawnActorfromClass "/Game/_TheCubeAssets/Blueprints/Levels/L_1-Waves/Waves-Barriers.Waves-Barriers_C" (Math|Transform|MakeTransform "0.000000,0.000000,-2200.000000") "AlwaysSpawn" "MultiplyWithRoot" 0 0))
            (bind _returnvalue_3 (Actor|GetActorOfClass "/Game/_TheCubeAssets/Blueprints/Levels/Blank.Blank_C"))
            (Transformation|AttachActorToActor _returnvalue_2 _returnvalue_3 "None" "KeepRelative" "KeepRelative" "KeepRelative" false)))))
    (else
      (return))))

(fn SpawnEnemiesOverTime
  (params (DT :type Float%20%28double-precision%29))
  ;[1 0.0307 0] Spawns Enemies Over Time instead of all at once
  (if (Math|Boolean|ANDBoolean (Variables|Default|GetRaiseComplete) (Variables|Default|GetRaise) (not (Variables|Default|GetSpawning%20Complete)))
    (if (> (Variables|Default|GetEnemiesDT) 1.0)
      (if (< (Variables|Default|GetEnemyCount) 10)
        (bind _returnvalue (Actor|GetActorOfClass "/Game/_TheCubeAssets/Blueprints/Levels/Blank.Blank_C" :!label _label))
        (for _index (range 0 4)
          (bind _random (CallFunction|RandomLocation))
          (bind _returnvalue_2 (Game|SpawnActorfromClass "/Game/_TheCubeAssets/Blueprints/Enemies/Ranged_Enemy.Ranged_Enemy_C" _random "AdjustIfPossibleButAlwaysSpawn" "MultiplyWithRoot" 0 0))
          (Transformation|AttachActorToActor _returnvalue_2 _returnvalue "None" "KeepRelative" "KeepRelative" "KeepRelative" true)
          (Math|Integer|IncrementInt (Variables|Default|GetEnemyCount)))
        (Variables|Default|SetEnemiesDT 0.0)
        (elif (> (stale _output_get) 2e+01)
          (if (< (Variables|Default|GetEnemyCount) 25)
            (goto _label)
            (else
              (Variables|Default|SetSpawning%20Complete true)))
          (else
            (Variables|Default|SetEnemiesDT (+ (stale _output_get) DT)))))
      (else
        (bind _output_get (Variables|Default|SetEnemiesDT (+ (Variables|Default|GetEnemiesDT) DT)))))))

(fn CheckifLevelEnded
  (if (Variables|Default|GetSpawning%20Complete)
    (bind _outactors (Actor|GetAllActorsOfClass "/Game/_TheCubeAssets/Blueprints/Enemies/Ranged_Enemy.Ranged_Enemy_C"))
    (bind _outactors_2 (Actor|GetAllActorsOfClass "/Game/_TheCubeAssets/Blueprints/Enemies/FlyingRanged_Enemy.FlyingRanged_Enemy_C"))
    (if (== (+ (Utilities|Array|Length _outactors_2) (Utilities|Array|Length _outactors)) 0)
      (bind _returnvalue (Actor|GetActorOfClass "/Game/_TheCubeAssets/Blueprints/LevelManager.LevelManager_C"))
      (Default|NextLevel _returnvalue))))

(fn GetLevelNumber
  (return (Variables|Components|GetLevel%20Number)))

(fn LevelEnded
  (bind _returnvalue (Actor|GetActorOfClass "/Game/_TheCubeAssets/Blueprints/LevelManager.LevelManager_C"))
  (Default|ClearBlankHolder _returnvalue)
  (if (Variables|Default|GetLevel%20In%20Progress)
    ;[0 1 0.4551] Show Objective
    (Development|PrintString (Utilities|String|Append (Utilities|String|Append "Level " (Utilities|String|ToString(Integer) (Variables|Components|GetLevel%20Number))) " ended!"))
    (bind _asgi_cube_game_instance (Utilities|Casting|CastToGI_CubeGameInstance (Game|GetGameInstance)))
    (bind _aswbp_hud (Utilities|Casting|CastToWBP_HUD (Variables|/Game/_TheCubeAssets/Blueprints/GI_CubeGameInstance.GI_CubeGameInstance_C|GetHUD%20Widget _asgi_cube_game_instance)))
    (Default|CompleteObjective _aswbp_hud (+ (Variables|Components|GetLevel%20Number) 1)))
  (Variables|Default|SetLevel%20In%20Progress false)
  (return))