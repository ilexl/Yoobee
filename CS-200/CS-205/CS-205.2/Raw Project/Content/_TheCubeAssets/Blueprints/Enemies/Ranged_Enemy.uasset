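; Ranged enemy Blueprint that attacks by firing projectiles on a reload cooldown.
; It sets max and current health in the construction script, and Tick accumulates the time since the last shot.
; Attack spawns a BP_EnemyProjectile at ShootLocation once that time exceeds ReloadTime, resets the timer, and returns whether it fired.
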(event EventBeginPlay
  (|CallParentFunction)
  (Variables|Default|SetReloadTime 5.0)
  (Variables|Default|SetTimeSinceLastShot 0.0))

(event Collision|EventActorBeginOverlap
  (params (OtherActor :type Actor%20Object%20Reference))
  (|CallParentFunction OtherActor) ; This node is disabled and will not be called.\nDrag off pins to build functionality.
)

(event EventTick
  (params (DeltaSeconds :type Float%20%28single-precision%29))
  (|CallParentFunction DeltaSeconds)
  (Variables|Default|SetTimeSinceLastShot (+ DeltaSeconds (Variables|Default|GetTimeSinceLastShot))))

(fn ConstructionScript
  (bind _output_get (Variables|Default|SetMaxHealth 1e+02))
  (Variables|Default|SetHealth _output_get)
  (|CallParentFunction))

(fn Attack
  (if (> (Variables|Default|GetTimeSinceLastShot) (Variables|Default|GetReloadTime))
    (Game|SpawnActorfromClass "/Game/_TheCubeAssets/Blueprints/Enemies/BP_EnemyProjectile.BP_EnemyProjectile_C" (Transformation|GetWorldTransform (Variables|Default|GetShoot%20Location)) "Undefined" "MultiplyWithRoot" 0 0)
    (Variables|Default|SetTimeSinceLastShot 0.0)
    (return true)
    (else
      (return false))))